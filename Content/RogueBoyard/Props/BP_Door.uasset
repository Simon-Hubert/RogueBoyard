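; BP_Door is a hidden door prop that plays opening and closing animations in front of a room camera, apparently as a transition.
; Opening attaches it to the assigned camera; timelines slide its relative location during each animation, then hide it and fire Opened or Closed dispatchers.
; Closing also detaches it when finished.
; A separate PlaceDoor step, not called here, tracks the camera at a set distance until time expires, then signals placement.
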(event `self.ReceiveBeginPlay`
  (bind _asgm_rogue (cast `/Game/RogueBoyard/Core/GM_Rogue` (`GameplayStatics.GetGameMode`)))
  (set `self.GM` _asgm_rogue)
  (`self.Set Visibility` false))

(event `CE_SetCam`
  (params (Camera :type "CameraActor Object Reference"))
  (set `self.RoomCamera` Camera))

(event `CE_OpenDoor`
  (`self.K2_AttachToActor` (`self.RoomCamera`) "None" "KeepRelative" "KeepRelative" "KeepRelative")
  (`self.K2_SetActorRelativeLocation` (0.0 0.0 0.0))
  (`self.K2_SetActorRelativeRotation` (struct))
  (`SkeletalMeshComponent.PlayAnimation` (`self.SkeletalMesh`) "/Game/RogueBoyard/GA/Assets/Meshs/Door/Animation_Porte_Montage.Animation_Porte_Montage" false)
  (`KismetSystemLibrary.PrintString` "Open")
  (`self.Set Visibility` true)
  (bind (_direction _speed) (`Timeline|_Open` :!via `PlayFromStart`)
    (:`Update`
      (`self.K2_SetActorRelativeLocation` (`KismetMathLibrary.VLerp` (15.0 0.0 0.0) (0.0 0.0 0.0) _speed)))
    (:`Finished`
      (`self.ED_Opened`)
      (`KismetSystemLibrary.PrintString` "FinishedOpening")
      (`self.Set Visibility` false))))

(event `CE_CloseDoor`
  (`SkeletalMeshComponent.PlayAnimation` (`self.SkeletalMesh`) "/Game/RogueBoyard/GA/Assets/Meshs/Door/Animation_PorteClose_Montage.Animation_PorteClose_Montage" false)
  (`KismetSystemLibrary.PrintString` "Close")
  (`self.Set Visibility` true)
  (bind (_direction _speed) (`Timeline|Timeline` :!via `PlayFromStart`)
    (:`Update`
      (`self.K2_SetActorRelativeLocation` (`KismetMathLibrary.VLerp` (10.0 0.0 0.0) (18.0 0.0 0.0) _speed)))
    (:`Finished`
      (`self.ED_Closed`)
      (`KismetSystemLibrary.PrintString` "FinishedClosing")
      (`self.Set Visibility` false)
      (`self.K2_DetachFromActor` "KeepRelative"))))

(fn `PlaceDoor`
  (bind _roomcamera (`self.RoomCamera`))
  (bind _returnvalue (`self.K2_GetActorRotation` _roomcamera))
  (set `self.CurrentTime` (+ (`self.CurrentTime`) 0.05))
  (if (>= (`self.CurrentTime`) (`self.TimeToPlace`))
    (`KismetSystemLibrary.K2_ClearAndInvalidateTimerHandle` (`self.TimerPlaceDoor`))
    (set `self.TimerPlaceDoor` (struct))
    (set `self.CurrentTime` 0.0)
    (`self.ED_DoorPlaced`)
    (else
      (`self.K2_SetActorLocation` (+ (`self.K2_GetActorLocation` _roomcamera) (* (`KismetMathLibrary.GetForwardVector` _returnvalue) (`self.DoorDistToCam`))) false true)
      (`self.K2_SetActorRotation` (`KismetMathLibrary.MakeRotator` (.roll _returnvalue) (.pitch _returnvalue) (.yaw _returnvalue))))))

(fn `Set Visibility`
  (params (bNewVisibility :type Boolean))
  (`SceneComponent.SetVisibility` (`self.SkeletalMesh`) bNewVisibility false))

(fn `UserConstructionScript`)