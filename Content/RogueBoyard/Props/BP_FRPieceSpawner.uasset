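; Prop actor that spawns a requested number of BP_FRCoin actors as a staggered burst at its own location.
; CE_SpawnCoins stores the count, fires the first coin immediately, then runs a short looping timer that clears itself once none remain.
; Each coin gets a random rotation, adjusts for collisions but always spawns, and triggers a Wwise coin sound from the loop.
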(event `CE_SpawnCoin`
  (`|SpawnActorFromClass` "/Game/RogueBoyard/Props/BP_FRCoin.BP_FRCoin_C" (`KismetMathLibrary.MakeTransform` (`self.K2_GetActorLocation`) (`KismetMathLibrary.RandomRotator` true)) "AdjustIfPossibleButAlwaysSpawn" "MultiplyWithRoot" null null))

(event `CE_SpawnCoins`
  (params (Nb :type Integer :default 0))
  (set `self.CoinsLeft` Nb)
  (`self.CE_CoinSpawnLoop`)
  (bind _returnvalue (`KismetSystemLibrary.K2_SetTimerDelegate` (delegate `CE_CoinSpawnLoop`) 0.12 true)))

(event `CE_CoinSpawnLoop`
  (if (<= (`self.CoinsLeft`) 0)
    (`KismetSystemLibrary.K2_ClearAndInvalidateTimerHandle` (stale `CE_SpawnCoins` _returnvalue))
    (else
      (`self.CE_SpawnCoin`)
      (`/Engine/EditorBlueprintResources/StandardMacros.DecrementInt` (`self.CoinsLeft`)
        (:`  `
          (`AkGameplayStatics.PostEvent` "/Game/WwiseAudio/Events/Default_Work_Unit/Items/Coin/Play_SFX_Item_Coins_Get.Play_SFX_Item_Coins_Get"))))))

(fn `UserConstructionScript`)