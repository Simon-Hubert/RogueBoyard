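; Grimoire prop that a RogueCharacter picks up by overlapping it while it is grounded, once initialized.
; Pickup switches the owner and binds to that character's push and death events.
; A push releases the book, while the death handler also returns it to its default position, with Wwise audio for loop, take and lose.
; Tick yaws it toward its movement direction; a sine bobbing snippet is unconnected.
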(event `self.ReceiveInit`
  (set `self.bInit` true)
  (`AkGameplayStatics.PostEvent` "/Game/WwiseAudio/Events/Default_Work_Unit/Interactables/GrimoireLoop.GrimoireLoop"))

(event `self.Root.OnComponentBeginOverlap`
  (params (OverlappedComponent :type "PrimitiveComponent Object Reference") (OtherActor :type "Actor Object Reference") (OtherComp :type "PrimitiveComponent Object Reference") (OtherBodyIndex :type Integer) (bFromSweep :type Boolean) (SweepResult :type "HitResult Structure (by ref)"))
  (bind _currentowner (`self.CurrentOwner`))
  (if (`self.bInit`)
    (bind _asrogue_character (cast `RogueCharacter` OtherActor))
    (if (`self.bGrounded`)
      (`self.SwitchOwner` _asrogue_character)
      (set `self.bGrounded` false)
      (`AkGameplayStatics.PostEvent` "/Game/WwiseAudio/Events/Default_Work_Unit/Interactables/Grimoire_Take.Grimoire_Take")
      (add `RogueCharacter.OnCharacterPushedEvent` _currentowner (delegate `OnOwnerPushed`))
      (add `RogueCharacter.OnCharacterDeathEvent` _currentowner (`|CreateDelegate` :!event `OnOwnerDied`)))))

(event `OnOwnerPushed`
  (bind _currentowner (`self.CurrentOwner`))
  (set `self.bGrounded` true)
  (remove `RogueCharacter.OnCharacterPushedEvent` _currentowner (delegate `OnOwnerPushed`))
  (remove `RogueCharacter.OnCharacterDeathEvent` _currentowner (delegate `OnOwnerDied`))
  (`self.SwitchOwner` null)
  (`AkGameplayStatics.PostEvent` "/Game/WwiseAudio/Events/Default_Work_Unit/Interactables/Grimoire_Lose.Grimoire_Lose"))

(event `OnOwnerDied`
  (bind _currentowner (`self.CurrentOwner`))
  (set `self.bGrounded` true)
  (remove `RogueCharacter.OnCharacterPushedEvent` _currentowner (delegate `OnOwnerPushed`))
  (remove `RogueCharacter.OnCharacterDeathEvent` _currentowner (delegate `OnOwnerDied`))
  (`self.K2_SetActorLocation` (`self.DefaultPos`))
  (`self.SwitchOwner` null)
  (`AkGameplayStatics.PostEvent` "/Game/WwiseAudio/Events/Default_Work_Unit/Interactables/Grimoire_Lose.Grimoire_Lose"))

(event `self.ReceiveTick`
  (params (DeltaSeconds :type "Float (single-precision)"))
  (bind _returnvalue (`self.K2_GetActorLocation`))
  (bind (_returnvalue_roll _returnvalue_pitch _returnvalue_yaw) (`KismetMathLibrary.BreakRotator` (`KismetMathLibrary.FindLookAtRotation` _returnvalue (+ (`KismetMathLibrary.Normal` (/ (- (`self.Last Pos`) _returnvalue) DeltaSeconds)) _returnvalue))))
  (`self.K2_SetActorRotation` (`KismetMathLibrary.MakeRotator` 0.0 0.0 _returnvalue_yaw))
  (set `self.Last Pos` _returnvalue))

(fn `UserConstructionScript`)