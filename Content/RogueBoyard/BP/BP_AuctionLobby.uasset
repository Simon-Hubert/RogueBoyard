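; BP_AuctionLobby is the auction lobby room Blueprint, driving the HUD as the room begins and ends.
; On BeginPlay it caches player 0's HUD as HUD_Rogue.
; BeginRoom hides the title card and starts the HUD room timer with MaxRoomTime, while EndRoom stops both the room and vote timers.
; No auction logic appears in its graphs.
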(event `self.ReceiveBeginPlay`
  (bind _ashud_rogue (cast `/Game/RogueBoyard/Core/HUD_Rogue` (`PlayerController.GetHUD` (`GameplayStatics.GetPlayerController` 0))))
  (set `self.HUD` _ashud_rogue))

(event `self.ReceiveBeginRoom`
  (`/Game/RogueBoyard/Core/HUD_Rogue.CE_HideTitleCardSimon` (`self.HUD`))
  (`/Game/RogueBoyard/Core/HUD_Rogue.CE_StartRoomTimer` (`self.HUD`) (`self.MaxRoomTime`)))

(event `self.ReceiveEndRoom`
  (`/Game/RogueBoyard/Core/HUD_Rogue.CE_EndRoomTimer` (`self.HUD`))
  (`/Game/RogueBoyard/Core/HUD_Rogue.CE_EndVoteTimer` (`self.HUD`)))

(fn `UserConstructionScript`)