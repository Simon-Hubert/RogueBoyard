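; BP_Trap is a trapdoor trap that opens for a set time and then closes, triggered by OpenTrap, Started or the Tab key.
; When CanUse allows, it plays the open animation at an adjustable rate and disables trap collision, then plays the closing animation and restores query-only collision.
; It then calls CoolDown; a Reusable check feeds a DoOnce, and a separate reuse Delay is left unconnected.
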(event `Key|Tab`
  (params (Key :type "Key Structure"))
  (bind _trap (`self.Trap`))
  (:`Pressed`
    (if (`self.canUse`) :!label _label
      (if (not (`self.Reusable`))
        (`/Engine/EditorBlueprintResources/StandardMacros.DoOnce` false
          (:`Completed`
            _)))
      (`SkeletalMeshComponent.PlayAnimation` _trap "/Game/RogueBoyard/GA/Assets/Meshs/msh_Trappe/TrapdoorAnim_Anim.TrapdoorAnim_Anim" false)
      (`SkeletalMeshComponent.SetPlayRate` _trap (`self.TimeAnimationTrap`))
      (`PrimitiveComponent.SetCollisionEnabled` (`self.CollisionTrap`) "NoCollision")
      (`KismetSystemLibrary.Delay` (`self.TimeTrapOpen`))
      (`SkeletalMeshComponent.PlayAnimation` (`self.Trap`) "/Game/RogueBoyard/GA/Assets/Meshs/msh_Trappe/TrappeAnimCLS.TrappeAnimCLS" false)
      (`PrimitiveComponent.SetCollisionEnabled` (`self.CollisionTrap`) "QueryOnly")
      (`self.CoolDown` 1.0))))

(event `self.OpenTrap`
  (goto _label))

(event `self.Started`
  (`self.OpenTrap`))

(fn `UserConstructionScript`)