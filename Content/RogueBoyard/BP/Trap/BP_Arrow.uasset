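; BP_Arrow is a trap projectile that damages any RogueCharacter it hits.
; Its construction script copies speed, gravity, bounce, friction and damage settings onto the ProjectileMovement component and the actor, and sets the arrow's lifespan.
; The BoxArrow overlap applies damage to the character without destroying the arrow, which persists until its lifespan expires.
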(event `self.ReceiveBeginPlay`)

(event `self.BoxArrow.OnComponentBeginOverlap`
  (params (OverlappedComponent :type "PrimitiveComponent Object Reference") (OtherActor :type "Actor Object Reference") (OtherComp :type "PrimitiveComponent Object Reference") (OtherBodyIndex :type Integer) (bFromSweep :type Boolean) (SweepResult :type "HitResult Structure (by ref)"))
  (bind _asrogue_character (cast `RogueCharacter` OtherActor))
  (`RogueCharacter.TakeDamage` _asrogue_character (`self.Damage`)))

(event `self.ProjectileMovement.OnComponentActivated`
  (params (Component :type "ActorComponent Object Reference") (bReset :type Boolean)))

(fn `UserConstructionScript`
  (bind _projectilemovement (`self.ProjectileMovement`))
  (set `ProjectileMovementComponent.InitialSpeed` (`self.Speed`) _projectilemovement)
  (set `ProjectileMovementComponent.ProjectileGravityScale` (`self.Projectile Gravity Scale`) _projectilemovement)
  (set `ProjectileMovementComponent.Bounciness` (`self.Bounciness`) _projectilemovement)
  (set `ProjectileMovementComponent.Friction` (`self.Friction`) _projectilemovement)
  (set `ProjectileMovementComponent.bShouldBounce` (`self.Should Bounce`) _projectilemovement)
  (set `self.Damage` (`self.Damage`))
  (`self.SetLifeSpan` (`self.In Lifespan`)))