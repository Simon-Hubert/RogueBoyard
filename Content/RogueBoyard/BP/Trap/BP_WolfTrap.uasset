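; BP_WolfTrap is a bear trap that snaps shut and damages characters who step into it.
; An overlap on the detection box while open clears IsOpen and plays the closing animation for any actor, then applies Damage only to BP_Character.
; Started plays the reopening montage on a closed trap from a saved time, and Stopped records montage position so reopening can resume.
; Nothing here sets IsOpen back to true.
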(event `self.ReceiveBeginPlay`)

(event `self.Started`
  (if (not (`self.IsOpen`))
    (`AnimInstance.Montage_PlayWithBlendIn` (`SkeletalMeshComponent.GetAnimInstance` (`self.BearTrap`)) "/Game/RogueBoyard/GA/Assets/Meshs/msh_Beartrap/BeartrapAnimOPN_Bones_Armature_ArmatureAction_001_Montage.BeartrapAnimOPN_Bones_Armature_ArmatureAction_001_Montage" (make `AlphaBlendArgs` "/Niagara/DefaultAssets/Curves/Templates/LinearRampUp.LinearRampUp") 1.0 "MontageLength" (`self.TimeStart`) true)))

(event `self.Stopped`
  (bind _returnvalue (`AnimInstance.Montage_GetPosition` (`SkeletalMeshComponent.GetAnimInstance` (`self.BearTrap`)) "/Game/RogueBoyard/GA/Assets/Meshs/msh_Beartrap/BeartrapAnimOPN_Bones_Armature_ArmatureAction_001_Montage.BeartrapAnimOPN_Bones_Armature_ArmatureAction_001_Montage"))
  (`KismetSystemLibrary.PrintString` (`KismetStringLibrary.Conv_DoubleToString` _returnvalue))
  (set `self.TimeStart` _returnvalue))

(event `self.BoxDetectionPlayer.OnComponentBeginOverlap`
  (params (OverlappedComponent :type "PrimitiveComponent Object Reference") (OtherActor :type "Actor Object Reference") (OtherComp :type "PrimitiveComponent Object Reference") (OtherBodyIndex :type Integer) (bFromSweep :type Boolean) (SweepResult :type "HitResult Structure (by ref)"))
  (if (`self.IsOpen`)
    (set `self.IsOpen` false)
    (`SkeletalMeshComponent.PlayAnimation` (`self.BearTrap`) "/Game/RogueBoyard/GA/Assets/Meshs/msh_Beartrap/BeartrapAnim_Anim_Bones_Armature_ArmatureAction_001.BeartrapAnim_Anim_Bones_Armature_ArmatureAction_001" false)
    (bind _asbp_character (cast `/Game/RogueBoyard/Core/BP_Character` OtherActor))
    (`RogueCharacter.TakeDamage` _asbp_character (`self.Damage`))))

(fn `UserConstructionScript`)