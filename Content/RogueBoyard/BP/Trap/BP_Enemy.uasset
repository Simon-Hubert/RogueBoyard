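; BP_Enemy is a trap enemy that chases nearby characters and pushes those in its push zone on contact, then destroys itself.
; A detection volume, scaled in the construction script, maintains a list of nearby characters.
; Tick selects a target by shortest recorded distance and moves toward it.
; Search movement runs only until a player is first found, as this graph never resets that flag.
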(event `self.PushZone.OnComponentBeginOverlap`
  (params (OverlappedComponent :type "PrimitiveComponent Object Reference") (OtherActor :type "Actor Object Reference") (OtherComp :type "PrimitiveComponent Object Reference") (OtherBodyIndex :type Integer) (bFromSweep :type Boolean) (SweepResult :type "HitResult Structure (by ref)"))
  ;[0.1427 0.1427 0.1427] Push Player
  (cast `/Game/RogueBoyard/Core/BP_Character` OtherActor)
  (`self.Push` (`PrimitiveComponent.GetOverlappingActors` (`self.PushZone`) "/Game/RogueBoyard/Core/BP_Character.BP_Character_C"))
  (`self.K2_DestroyActor`))

(event `self.DetectPlayerAround.OnComponentBeginOverlap`
  (params (OverlappedComponent :type "PrimitiveComponent Object Reference") (OtherActor :type "Actor Object Reference") (OtherComp :type "PrimitiveComponent Object Reference") (OtherBodyIndex :type Integer) (bFromSweep :type Boolean) (SweepResult :type "HitResult Structure (by ref)"))
  ;[0.09271 0.09271 0.09271] List PlayerAround
  (bind _asbp_character (cast `/Game/RogueBoyard/Core/BP_Character` OtherActor))
  (`KismetArrayLibrary.Array_Add` (`self.ListCloseEnemies`) _asbp_character))

(event `self.DetectPlayerAround.OnComponentEndOverlap`
  (params (OverlappedComponent :type "PrimitiveComponent Object Reference") (OtherActor :type "Actor Object Reference") (OtherComp :type "PrimitiveComponent Object Reference") (OtherBodyIndex :type Integer))
  ;[0.09271 0.09271 0.09271] List PlayerAround
  (bind _asbp_character (cast `/Game/RogueBoyard/Core/BP_Character` OtherActor))
  (`KismetArrayLibrary.Array_RemoveItem` (`self.ListCloseEnemies`) _asbp_character)
  (if (== OtherActor (`self.CloserPlayer`))
    (set `self.CloserPlayer` null)
    (set `self.DistancePlayerCloser` 500000000.0)))

(event `self.ReceiveTick`
  (params (DeltaSeconds :type "Float (single-precision)"))
  ;[0.1594 0.1594 0.1594] Move and Rotate to Player
  (for _array_element (`self.ListCloseEnemies`)
    (bind _returnvalue (`self.GetDistanceTo` _array_element self))
    (if (> (`self.DistancePlayerCloser`) _returnvalue)
      (set `self.DistancePlayerCloser` _returnvalue)
      (bind _output_get (set `self.CloserPlayer` _array_element))))
  (`/Engine/EditorBlueprintResources/StandardMacros.IsValid` _output_get
    (:`Is Valid`
      (set `self.PlayerFound` true)
      (`self.MoveToPlayer` (`self.CloserPlayer`) DeltaSeconds))
    (:`Is Not Valid`
      (if (not (`self.PlayerFound`))
        (`self.SearchMovement` DeltaSeconds)))))

(fn `UserConstructionScript`
  (bind _detectplayeraround (`self.DetectPlayerAround`))
  (`SceneComponent.SetWorldScale3D` _detectplayeraround (* (`SceneComponent.K2_GetComponentScale` _detectplayeraround) (`self.SizeBoxDetectingPlayer`))))