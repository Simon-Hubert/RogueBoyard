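; BP_LargeBall is a trap ball that a player steers between four corner points of a square.
; Joystick direction events, mirrored by keyboard keys, use PosPlayer as the current corner index and allow only moves to the adjacent corner in that direction.
; Each move stores the corner component's world X/Y, with Z zeroed, in PosToMove.
; Tick passes any non-zero PosToMove to MoveTowardsTarget to drive the movement.
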(event `self.ReceiveTick`
  (params (DeltaSeconds :type "Float (single-precision)"))
  (bind _postomove (`self.PosToMove`))
  (if (!= _postomove (0.0 0.0 0.0))
    (`self.MoveTowardsTarget` DeltaSeconds _postomove)))

(event `self.JoystickMoveUp`
  (bind (_returnvalue_x _returnvalue_y) (`KismetMathLibrary.BreakVector` (`SceneComponent.K2_GetComponentLocation` (`self.TopLeft`))))
  (bind (_returnvalue_x_2 _returnvalue_y_2) (`KismetMathLibrary.BreakVector` (`SceneComponent.K2_GetComponentLocation` (`self.TopRight`))))
  (if (== (`self.PosPlayer`) 0) :!label _label
    (set `self.PosToMove` (`KismetMathLibrary.MakeVector` _returnvalue_x _returnvalue_y))
    (set `self.PosPlayer` 2)
    (elif (== (`self.PosPlayer`) 1)
      (set `self.PosToMove` (`KismetMathLibrary.MakeVector` _returnvalue_x_2 _returnvalue_y_2))
      (set `self.PosPlayer` 3))))

(event `Key|O`
  (params (Key :type "Key Structure"))
  (:`Pressed`
    (goto _label)))

(event `self.JoystickMoveDown`
  (bind (_returnvalue_x _returnvalue_y) (`KismetMathLibrary.BreakVector` (`SceneComponent.K2_GetComponentLocation` (`self.DownLeft`))))
  (bind (_returnvalue_x_2 _returnvalue_y_2) (`KismetMathLibrary.BreakVector` (`SceneComponent.K2_GetComponentLocation` (`self.DownRight`))))
  (if (== (`self.PosPlayer`) 2) :!label _label_2
    (set `self.PosToMove` (`KismetMathLibrary.MakeVector` _returnvalue_x _returnvalue_y))
    (set `self.PosPlayer` 0)
    (elif (== (`self.PosPlayer`) 3)
      (set `self.PosToMove` (`KismetMathLibrary.MakeVector` _returnvalue_x_2 _returnvalue_y_2))
      (set `self.PosPlayer` 1))))

(event `Key|L`
  (params (Key :type "Key Structure"))
  (:`Pressed`
    (goto _label_2)))

(event `self.JoystickMoveRight`
  (bind (_returnvalue_x _returnvalue_y) (`KismetMathLibrary.BreakVector` (`SceneComponent.K2_GetComponentLocation` (`self.DownRight`))))
  (bind (_returnvalue_x_2 _returnvalue_y_2) (`KismetMathLibrary.BreakVector` (`SceneComponent.K2_GetComponentLocation` (`self.TopRight`))))
  (if (== (`self.PosPlayer`) 0) :!label _label_3
    (set `self.PosToMove` (`KismetMathLibrary.MakeVector` _returnvalue_x _returnvalue_y))
    (set `self.PosPlayer` 1)
    (elif (== (`self.PosPlayer`) 2)
      (set `self.PosToMove` (`KismetMathLibrary.MakeVector` _returnvalue_x_2 _returnvalue_y_2))
      (set `self.PosPlayer` 3))))

(event `Key|M`
  (params (Key :type "Key Structure"))
  (:`Pressed`
    (goto _label_3)))

(event `self.JoystickMoveLeft`
  (bind (_returnvalue_x _returnvalue_y) (`KismetMathLibrary.BreakVector` (`SceneComponent.K2_GetComponentLocation` (`self.TopLeft`))))
  (bind (_returnvalue_x_2 _returnvalue_y_2) (`KismetMathLibrary.BreakVector` (`SceneComponent.K2_GetComponentLocation` (`self.DownLeft`))))
  (if (== (`self.PosPlayer`) 1) :!label _label_4
    (set `self.PosToMove` (`KismetMathLibrary.MakeVector` _returnvalue_x_2 _returnvalue_y_2))
    (set `self.PosPlayer` 0)
    (elif (== (`self.PosPlayer`) 3)
      (set `self.PosToMove` (`KismetMathLibrary.MakeVector` _returnvalue_x _returnvalue_y))
      (set `self.PosPlayer` 2))))

(event `Key|K`
  (params (Key :type "Key Structure"))
  (:`Pressed`
    (goto _label_4)))

(fn `UserConstructionScript`)