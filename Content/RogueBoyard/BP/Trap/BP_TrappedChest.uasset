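; BP_TrappedChest is a mimic chest trap that damages characters standing in its attack zone.
; On BeginPlay it holds the mimic animation at zero play rate.
; Interact, or a Tab key press sharing the same path, checks CanUse, then plays the animation at SpeedAnimation.
; It applies Damage to each BP_Character overlapping ZoneAttack and calls a fixed-length CoolDown.
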(event `self.ReceiveBeginPlay`
  (bind _sk_chest (`self.SK_Chest`))
  (`SkeletalMeshComponent.PlayAnimation` _sk_chest "/Game/RogueBoyard/GA/Assets/Meshs/msh_Mimic/MimicAnimationV01_Anim.MimicAnimationV01_Anim" false)
  (`SkeletalMeshComponent.SetPlayRate` _sk_chest 0.0))

(event `/Game/RogueBoyard/BP/I_Interactable.Interact`
  (bind _sk_chest (`self.SK_Chest`))
  (if (`self.canUse`) :!label _label
    (`SkeletalMeshComponent.PlayAnimation` _sk_chest "/Game/RogueBoyard/GA/Assets/Meshs/msh_Mimic/MimicAnimationV01_Anim.MimicAnimationV01_Anim" false)
    (`SkeletalMeshComponent.SetPlayRate` _sk_chest (`self.SpeedAnimation`))
    (for _array_element (`PrimitiveComponent.GetOverlappingActors` (`self.ZoneAttack`) "/Game/RogueBoyard/Core/BP_Character.BP_Character_C")
      (bind _asbp_character (cast `/Game/RogueBoyard/Core/BP_Character` _array_element))
      (`RogueCharacter.TakeDamage` _asbp_character (`self.Damage`)))
    (`self.CoolDown` 3.0)))

(event `Key|Tab`
  (params (Key :type "Key Structure"))
  (:`Pressed`
    (goto _label)))

(fn `UserConstructionScript`)