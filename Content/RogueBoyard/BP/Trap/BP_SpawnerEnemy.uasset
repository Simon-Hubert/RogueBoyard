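; BP_SpawnerEnemy is a trap that spawns a batch of BP_Enemy actors when started or when Tab is pressed.
; If CanUse is set, it spawns NEnemyToSpawn enemies in one loop, adjusting for collisions, then calls a five-second CoolDown.
; The construction script sizes the ZoneSpawn box from SizeZoneSpawn, but the random-point-in-box node is unused and the between-spawn delay never runs.
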(event `Key|Tab`
  (params (Key :type "Key Structure"))
  (:`Pressed`
    (if (`self.canUse`) :!label _label
      (for _ (range 1 (+ (`self.NEnemyToSpawn`) 1))
        (`|SpawnActorFromClass` "/Game/RogueBoyard/BP/Trap/BP_Enemy.BP_Enemy_C" (`KismetMathLibrary.MakeTransform` (0.0 0.0 0.0)) "AdjustIfPossibleButAlwaysSpawn" "OverrideRootScale" null null))
      (`self.CoolDown` 5.0))))

(event `self.Started`
  (goto _label))

(fn `UserConstructionScript`
  (bind _sizezonespawn (`self.SizeZoneSpawn`))
  (`BoxComponent.SetBoxExtent` (`self.ZoneSpawn`) (`KismetMathLibrary.MakeVector` _sizezonespawn _sizezonespawn 32.0) true))