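; BP_Blackhole is a trap that applies attraction to characters inside its sphere zone.
; Overlap events on the Zone add and remove BP_Character actors from a player list, printing a debug string on entry.
; Every tick, it calls AttractPlayers on each listed player, passing distance from the center divided by the sphere radius, clamped so the value rises from zero at the center to one at the edge.
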(event `self.ReceiveTick`
  (params (DeltaSeconds :type "Float (single-precision)"))
  (for _array_element (`self.ListPlayer`)
    (`self.AttractPlayers` (`KismetMathLibrary.FClamp` (/ (`KismetMathLibrary.Vector_Distance` (`self.K2_GetActorLocation` _array_element) (`self.K2_GetActorLocation`)) (`SphereComponent.GetScaledSphereRadius` (`self.Zone`)))) _array_element)))

(event `self.Zone.OnComponentBeginOverlap`
  (params (OverlappedComponent :type "PrimitiveComponent Object Reference") (OtherActor :type "Actor Object Reference") (OtherComp :type "PrimitiveComponent Object Reference") (OtherBodyIndex :type Integer) (bFromSweep :type Boolean) (SweepResult :type "HitResult Structure (by ref)"))
  (bind _asbp_character (cast `/Game/RogueBoyard/Core/BP_Character` OtherActor))
  (`KismetSystemLibrary.PrintString` "Blackhole")
  (`KismetArrayLibrary.Array_Add` (`self.ListPlayer`) _asbp_character))

(event `self.Zone.OnComponentEndOverlap`
  (params (OverlappedComponent :type "PrimitiveComponent Object Reference") (OtherActor :type "Actor Object Reference") (OtherComp :type "PrimitiveComponent Object Reference") (OtherBodyIndex :type Integer))
  (bind _asbp_character (cast `/Game/RogueBoyard/Core/BP_Character` OtherActor))
  (`KismetArrayLibrary.Array_RemoveItem` (`self.ListPlayer`) _asbp_character))

(fn `UserConstructionScript`)