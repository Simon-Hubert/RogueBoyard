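; BP_Wallblade is a blade trap that damages any BP_Character that begins overlapping its Box, using the Damage value.
; The construction script sizes the trap from MaxDistance, placing two arrows at opposite ends along local Y and stretching the LameRail on X to match.
; The graphs shown contain no logic that moves the blade.
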(event `self.Box.OnComponentBeginOverlap`
  (params (OverlappedComponent :type "PrimitiveComponent Object Reference") (OtherActor :type "Actor Object Reference") (OtherComp :type "PrimitiveComponent Object Reference") (OtherBodyIndex :type Integer) (bFromSweep :type Boolean) (SweepResult :type "HitResult Structure (by ref)"))
  (bind _asbp_character (cast `/Game/RogueBoyard/Core/BP_Character` OtherActor))
  (`RogueCharacter.TakeDamage` _asbp_character (`self.Damage`)))

(fn `UserConstructionScript`
  (bind _maxdistance (`self.MaxDistance`))
  (`SceneComponent.K2_SetRelativeLocation` (`self.Arrow`) (`KismetMathLibrary.MakeVector` 0.0 _maxdistance 50.0) false false)
  (`SceneComponent.K2_SetRelativeLocation` (`self.Arrow1`) (`KismetMathLibrary.MakeVector` 0.0 (* _maxdistance -1.0) 50.0) false false)
  (`SceneComponent.SetRelativeScale3D` (`self.Lame_Rail`) (`KismetMathLibrary.MakeVector` (/ _maxdistance 24.0) 1.0 1.0)))