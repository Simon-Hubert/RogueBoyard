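; Millstone trap actor that spins around a pivot and damages any BP_Character that overlaps its box.
; BeginPlay reads each cylinder's offset and calls CalculateSpeedRotation to set per-cylinder roll speeds, apparently meant to scale with offset over pivot height.
; Once Init enables motion and posts the grindstone loop sound, Tick yaws the pivot and pitches the six cylinders, negating both for counter-clockwise rotation.
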(event `self.ReceiveBeginPlay`
  (bind (_relativelocation_x _relativelocation_y) (`KismetMathLibrary.BreakVector` (`SceneComponent.RelativeLocation` (`self.MillestoneCylinderInt`))))
  (bind (_relativelocation_x_2 _relativelocation_y_2) (`KismetMathLibrary.BreakVector` (`SceneComponent.RelativeLocation` (`self.MillestoneCylinder3`))))
  (bind (_relativelocation_x_3 _relativelocation_y_3) (`KismetMathLibrary.BreakVector` (`SceneComponent.RelativeLocation` (`self.MillestoneCylinderExt`))))
  (bind (_relativelocation_x_4 _relativelocation_y_4) (`KismetMathLibrary.BreakVector` (`SceneComponent.RelativeLocation` (`self.MillestoneCylinder1`))))
  (bind (_relativelocation_x_5 _relativelocation_y_5 _relativelocation_z) (`KismetMathLibrary.BreakVector` (`SceneComponent.RelativeLocation` (`self.PivotRotation`))))
  (bind (_relativelocation_x_6 _relativelocation_y_6) (`KismetMathLibrary.BreakVector` (`SceneComponent.RelativeLocation` (`self.MillestoneCylinder4`))))
  (bind (_relativelocation_x_7 _relativelocation_y_7) (`KismetMathLibrary.BreakVector` (`SceneComponent.RelativeLocation` (`self.MillestoneCylinder2`))))
  (set `self.DCylinder1` _relativelocation_y_4)
  (set `self.DCylinder2` _relativelocation_y_7)
  (set `self.DCylinder3` _relativelocation_y_2)
  (set `self.DCylinder4` _relativelocation_y_6)
  (set `self.DCylinderExt` _relativelocation_y_3)
  (set `self.DCylinderInt` _relativelocation_y)
  (set `self.RCylinder` _relativelocation_z)
  (set `self.SCylinderInt` (`self.CalculateSpeedRotation` (`self.DCylinderInt`)))
  (set `self.SCylinder1` (`self.CalculateSpeedRotation` (`self.DCylinder1`)))
  (set `self.SCylinder2` (`self.CalculateSpeedRotation` (`self.DCylinder2`)))
  (set `self.SCylinder3` (`self.CalculateSpeedRotation` (`self.DCylinder3`)))
  (set `self.SCylinder4` (`self.CalculateSpeedRotation` (`self.DCylinder4`)))
  (set `self.SCylinderExt` (`self.CalculateSpeedRotation` (`self.DCylinderExt`))))

(event `self.ReceiveTick`
  (params (DeltaSeconds :type "Float (single-precision)"))
  (set `self.Delta Seconds` DeltaSeconds)
  (if (`self.IsInit`)
    (if (`self.ClockwiseRotation`)
      (`SceneComponent.K2_AddLocalRotation` (`self.PivotRotation`) (`KismetMathLibrary.MakeRotator` 0.0 0.0 (* (`self.SpeedRotation`) (`self.Delta Seconds`))) false false)
      (`self.SetRotation` (`self.SCylinderInt`) (`self.MillestoneCylinderInt`))
      (`self.SetRotation` (`self.SCylinder1`) (`self.MillestoneCylinder1`))
      (`self.SetRotation` (`self.SCylinder2`) (`self.MillestoneCylinder2`))
      (`self.SetRotation` (`self.SCylinder3`) (`self.MillestoneCylinder3`))
      (`self.SetRotation` (`self.SCylinder4`) (`self.MillestoneCylinder4`))
      (`self.SetRotation` (`self.SCylinderExt`) (`self.MillestoneCylinderExt`))
      (else
        (`SceneComponent.K2_AddLocalRotation` (`self.PivotRotation`) (`KismetMathLibrary.MakeRotator` 0.0 0.0 (* (* (`self.SpeedRotation`) -1.0) (`self.Delta Seconds`))) false false)
        (`self.SetRotation` (* (`self.SCylinderInt`) -1.0) (`self.MillestoneCylinderInt`))
        (`self.SetRotation` (* (`self.SCylinder1`) -1.0) (`self.MillestoneCylinder1`))
        (`self.SetRotation` (* (`self.SCylinder2`) -1.0) (`self.MillestoneCylinder2`))
        (`self.SetRotation` (* (`self.SCylinderExt`) -1.0) (`self.MillestoneCylinderExt`))
        (`self.SetRotation` (* (`self.SCylinder3`) -1.0) (`self.MillestoneCylinder3`))
        (`self.SetRotation` (* (`self.SCylinder4`) -1.0) (`self.MillestoneCylinder4`))))))

(event `self.ReceiveInit`
  (set `self.IsInit` true)
  (`AkGameplayStatics.PostEvent` "/Game/WwiseAudio/Events/Default_Work_Unit/Traps/GrindStone/Play_SFX_Trap_Grindstone_LP.Play_SFX_Trap_Grindstone_LP"))

(event `self.Box.OnComponentBeginOverlap`
  (params (OverlappedComponent :type "PrimitiveComponent Object Reference") (OtherActor :type "Actor Object Reference") (OtherComp :type "PrimitiveComponent Object Reference") (OtherBodyIndex :type Integer) (bFromSweep :type Boolean) (SweepResult :type "HitResult Structure (by ref)"))
  (bind _asbp_character (cast `/Game/RogueBoyard/Core/BP_Character` OtherActor))
  (`RogueCharacter.TakeDamage` _asbp_character (`self.Damage`)))

(fn `SetRotation`
  (params (A :type "Float (double-precision)") (self2 :type "SceneComponent Object Reference") (NewParam :type Boolean))
  (bind (_relativerotation_roll _relativerotation_pitch _relativerotation_yaw) (`KismetMathLibrary.BreakRotator` (`SceneComponent.RelativeRotation` self2)))
  (if (> _relativerotation_pitch 360.0)
    (`SceneComponent.K2_SetRelativeRotation` self2 (`KismetMathLibrary.MakeRotator` _relativerotation_roll 0.0 _relativerotation_yaw) false false))
  (`SceneComponent.K2_AddLocalRotation` self2 (`KismetMathLibrary.MakeRotator` 0.0 (* A (`self.Delta Seconds`))) false false))

(fn `UserConstructionScript`)