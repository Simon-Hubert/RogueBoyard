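; BP_Crossbow is a chargeable crossbow trap that fires BP_Arrow projectiles.
; Started or the O key begins a charge if usable and starts a cooldown; Stopped or P releases it through a re-armed DoOnce.
; Tick builds Power up to ChargeTime, driving the Niagara charge effect and switching it at full charge.
; Release spawns an arrow along DirectionalArrow with speed scaled by Power, and plays a Wwise sound.
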(event `CE_FinishedCharging`
  (`NiagaraComponent.SetAsset` (`self.Niagara`) "/Game/RogueBoyard/VFX/Systems/Arbalete/NS_CrossbowFullyCharged.NS_CrossbowFullyCharged" true))

(event `self.ReceiveBeginPlay`
  (bind _returnvalue (`GameplayStatics.GetActorOfClass` "/Game/RogueBoyard/BP/Trap/BP_Arrow.BP_Arrow_C"))
  (set `self.CrossbowArrow` _returnvalue))

(event `self.ReceiveInit`
  (set `self.Initialized` true))

(event `self.ReceiveTick`
  (params (DeltaSeconds :type "Float (single-precision)"))
  (`self.Update` DeltaSeconds))

(event `Key|O`
  (params (Key :type "Key Structure"))
  (:`Pressed`
    (if (`self.canUse`) :!label _label
      (`self.CoolDown` 2.0)
      (bind _newparam (`self.StartCharging`))
      (if _newparam
        (goto _label_2 :!via `Reset`)))))

(event `self.Started`
  (if (`self.Initialized`)
    (goto _label)))

(event `Key|P`
  (params (Key :type "Key Structure"))
  (:`Pressed`
    (`/Engine/EditorBlueprintResources/StandardMacros.DoOnce` true :!label _label_2
      (:`Completed`
        (`self.ReleaseShot`)
        (set `self.Charging` false)))))

(event `self.Stopped`
  (if (`self.Initialized`)
    (goto _label_2)))

(event `self.ReleaseShot`
  (if (`self.Initialized`)
    (`SceneComponent.SetVisibility` (`self.Niagara`) false false)
    (`self.Shoot`)
    (`AkGameplayStatics.PostEvent` "/Game/WwiseAudio/Events/Default_Work_Unit/Traps/Crossbow/Play_Crossbow.Play_Crossbow")))

(fn `Shoot`
  (`|SpawnActorFromClass` "/Game/RogueBoyard/BP/Trap/BP_Arrow.BP_Arrow_C" (`SceneComponent.K2_GetComponentToWorld` (`self.DirectionalArrow`)) "Undefined" "MultiplyWithRoot" null (`KismetMathLibrary.Lerp` (`self.MinimalSpeed`) (`self.Max Speed`) (`self.power`)) (`self.In Lifespan`) 0.0 0.0 0.0 false (`self.Damage`) null))

(fn `StartCharging`
  (returns (NewParam :type Boolean))
  (bind _niagara (`self.Niagara`))
  (if (not (`self.Charging`))
    (set `self.Charging` true)
    (set `self.elapsedTime` 0.0)
    (`NiagaraComponent.SetAsset` _niagara "/Game/RogueBoyard/VFX/Systems/Arbalete/NS_CrossbowCharge.NS_CrossbowCharge" true)
    (`SceneComponent.SetVisibility` _niagara true false)
    (return true)
    (else
      (return false))))

(fn `Update`
  (params (DeltaTime :type "Float (double-precision)"))
  (bind _elapsedtime (`self.elapsedTime`))
  (bind _chargetime (`self.ChargeTime`))
  (if (`self.Charging`)
    (set `self.elapsedTime` (`KismetMathLibrary.FClamp` (+ DeltaTime (`self.elapsedTime`)) 0.0 (`self.ChargeTime`)))
    (bind _output_get (set `self.power` (/ _elapsedtime _chargetime)))
    (`NiagaraComponent.SetVariableFloat` (`self.Niagara`) "ChargePercent" _output_get)
    (if (>= _elapsedtime _chargetime)
      (`self.CE_FinishedCharging`))))

(fn `UserConstructionScript`)