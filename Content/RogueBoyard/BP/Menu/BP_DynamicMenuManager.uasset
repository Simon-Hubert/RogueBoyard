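; BP_DynamicMenuManager sets up the main menu at play start and provides a helper for playing level sequences.
; On BeginPlay it calls CEInit on the HUD_MainMenu of player 0, then switches that player's view to the title screen camera.
; PlayLevelSequence creates a player for the given sequence, binds the supplied callback to its stop event and plays it.
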(event `self.ReceiveBeginPlay`
  (`self.InitHUD`)
  (`PlayerController.SetViewTargetWithBlend` (`GameplayStatics.GetPlayerController` 0) (`self.CamTitleScreen`) 0.0 "VTBlend_Linear" 0.0 false))

(fn `InitHUD`
  (bind _ashud_main_menu (cast `/Game/RogueBoyard/Core/HUD_MainMenu` (`PlayerController.GetHUD` (`GameplayStatics.GetPlayerController` 0))))
  (`/Game/RogueBoyard/Core/HUD_MainMenu.CE_Init` _ashud_main_menu))

(fn `Play Level Sequence`
  (params (BindToOnStop :type "Object Object Reference (by ref)") (Sequence :type "LevelSequence Object Reference"))
  (bind (_outactor _returnvalue) (`LevelSequencePlayer.CreateLevelSequencePlayer` Sequence))
  (add `MovieSceneSequencePlayer.OnStop` _returnvalue BindToOnStop)
  (`MovieSceneSequencePlayer.Play` _returnvalue))

(fn `UserConstructionScript`)