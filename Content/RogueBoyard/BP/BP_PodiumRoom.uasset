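; End-of-game podium room that ranks players by purse, shows the winner on the HUD, then the end-game screen after timed delays.
; It registers with GM_Rogue, bubble-sorts player index and purse pairs packed into vectors, and spawns posed BP_Statues colored from DT_Character for all but last place.
; The fourth-ranked character is teleported to the fourth spot with the room camera, while other characters switch to a Waiting state.
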(event `self.ReceiveBeginPlay`
  (bind _asgm_rogue (cast `/Game/RogueBoyard/Core/GM_Rogue` (`GameplayStatics.GetGameMode`)))
  (set `/Game/RogueBoyard/Core/GM_Rogue.PodiumManager` self _asgm_rogue)
  (set `self.As GM Rogue` _asgm_rogue)
  (bind _ashud_rogue (cast `/Game/RogueBoyard/Core/HUD_Rogue` (`PlayerController.GetHUD` (`GameplayStatics.GetPlayerController` 0))))
  (set `self.HUD` _ashud_rogue))

(event `self.ReceiveRoomEnter`
  (bind _output_x (`KismetMathLibrary.BreakVector` (`|GetArrayItem` (`self.Players`))))
  (`self.SortArray` (`PlayerStatSubsystem.GetPlayerPurses` (subsystem `PlayerStatSubsystem`)))
  (`self.SpawnStatues`)
  (`/Game/RogueBoyard/Core/HUD_Rogue.CE_ShowWinner` (`self.HUD`) (`KismetMathLibrary.FTrunc` _output_x))
  (`KismetSystemLibrary.Delay` 3.0)
  (`self.BeginRoom`))

(event `self.ReceiveBeginRoom`
  (bind _output_x (`KismetMathLibrary.BreakVector` (`|GetArrayItem` (`self.Players`) 3)))
  (bind _output (`|GetArrayItem` (`RogueGameMode.Characters` (`self.As GM Rogue`)) (`KismetMathLibrary.FTrunc` _output_x)))
  (`self.K2_SetActorLocation` _output (`SceneComponent.K2_GetComponentLocation` (`self.Fourth`)) false true)
  (`self.MakeCharWaiting`)
  (`RogueCharacter.SetCameraByParam` _output (`self.RoomCamera`))
  (`KismetSystemLibrary.Delay` 7.0)
  (`/Game/RogueBoyard/Core/HUD_Rogue.CE_ShowEndGame` (`self.HUD`)))

(fn `GetStatue`
  (params (PlayerIndex :type Integer))
  (returns (Statue :type "StaticMesh Object Reference"))
  (switch `int` PlayerIndex
    (:`0`
      (return "/Game/RogueBoyard/GA/Assets/Meshs/Satue/PEEZZY_Pose_Blue.PEEZZY_Pose_Blue"))
    (:`1`
      (return "/Game/RogueBoyard/GA/Assets/Meshs/Satue/SKWEEZZY_Pose_Purple.SKWEEZZY_Pose_Purple"))
    (:`2`
      (return "/Game/RogueBoyard/GA/Assets/Meshs/Satue/Izzy_pose_Green.Izzy_pose_Green"))
    (:`3`
      (return "/Game/RogueBoyard/GA/Assets/Meshs/Satue/Lizard_Wizard_Figurine.Lizard_Wizard_Figurine"))))

(fn `GetTransformPodium`
  (params (Order :type Integer))
  (returns (Transform :type "Transform Structure"))
  (switch `int` Order
    (:`0`
      (return (`SceneComponent.K2_GetComponentToWorld` (`self.First`))))
    (:`1`
      (return (`SceneComponent.K2_GetComponentToWorld` (`self.Second`))))
    (:`2`
      (return (`SceneComponent.K2_GetComponentToWorld` (`self.Third`))))
    (:`3`
      (return (`SceneComponent.K2_GetComponentToWorld` (`self.Fourth`))))))

(fn `MakeCharWaiting`
  (bind _output_x (`KismetMathLibrary.BreakVector` (`|GetArrayItem` (`self.Players`) 3)))
  (for _array_element (`RogueGameMode.Characters` (`self.As GM Rogue`))
    (if (!= (`RogueCharacter.PlayerIndex` _array_element) (`KismetMathLibrary.FTrunc` _output_x))
      (`RogueCharacterStateMachine.ChangeState` (`RogueCharacter.StateMachine` _array_element) "Waiting"))))

(fn `SortArray`
  (params (InArray :type "Array of Integer"))
  (bind _players (`self.Players`))
  (bind _returnvalue (- (`KismetArrayLibrary.Array_Length` _players) 2))
  (for (_array_element _array_index) InArray
    (`KismetArrayLibrary.Array_Add` _players (`KismetMathLibrary.MakeVector` (`KismetMathLibrary.Conv_IntToDouble` _array_index) (`KismetMathLibrary.Conv_IntToDouble` _array_element))))
  (for _ (range (+ _returnvalue 1))
    (for _index (range (+ _returnvalue 1))
      (bind (_output_x _output_y) (`KismetMathLibrary.BreakVector` (`|GetArrayItem` _players _index)))
      (bind _returnvalue_2 (+ _index 1))
      (bind (_output_x_2 _output_y_2) (`KismetMathLibrary.BreakVector` (`|GetArrayItem` _players _returnvalue_2)))
      (if (< _output_y _output_y_2)
        (`KismetArrayLibrary.Array_Swap` _players _index _returnvalue_2)))))

(fn `SpawnStatues`
  (bind _players (`self.Players`))
  (for (_array_element _array_index) _players
    (if (not (== _array_index (- (`KismetArrayLibrary.Array_Length` _players) 1)))
      (bind _returnvalue (`KismetMathLibrary.FTrunc` (.x _array_element)))
      (bind _statue (`self.GetStatue` _returnvalue))
      (bind _transform (`self.GetTransformPodium` _array_index))
      (bind _returnvalue_2 (`|SpawnActorFromClass` "/Game/RogueBoyard/GA/Assets/Meshs/Satue/BP_Statue.BP_Statue_C" _transform "Undefined" "MultiplyWithRoot" null null))
      (`StaticMeshComponent.SetStaticMesh` (`/Game/RogueBoyard/GA/Assets/Meshs/Satue/BP_Statue.StaticMesh` _returnvalue_2) _statue)
      (bind _outrownames (`DataTableFunctionLibrary.GetDataTableRowNames` "/Game/RogueBoyard/Characters/DT_Character.DT_Character"))
      (bind _returnvalue_3 (`|GetDataTableRow` "/Game/RogueBoyard/Characters/DT_Character.DT_Character" (`|GetArrayItem` _outrownames _returnvalue))
        (:`then`
          (set `/Game/RogueBoyard/GA/Assets/Meshs/Satue/BP_Statue.Color` (`.Player_Color_5_B78D15C3476A269E83BACD8E20EF06D1` (break `/Game/RogueBoyard/Characters/ST_Player` _returnvalue_3)) _returnvalue_2)
          (bind _output_get (set `/Game/RogueBoyard/GA/Assets/Meshs/Satue/BP_Statue.PlayerIndex` _returnvalue _returnvalue_2))
          (`/Game/RogueBoyard/GA/Assets/Meshs/Satue/BP_Statue.BeginAnim` _returnvalue_2 _output_get))))))

(fn `UserConstructionScript`)