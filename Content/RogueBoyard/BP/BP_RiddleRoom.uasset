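; Riddle room controller for a lever-deactivation escape challenge, running the room's flow from entry to exit.
; On enter it shows the HUD title card, sets the door camera, places players and opens the BP_Door, whose opened event starts the chrono, then the timed room and every RogueTrap.
; Ending stops timer and traps, shows the result, then closes the door, whose closed event triggers RoomExit.
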(event `self.ReceiveBeginPlay`
  (bind _ashud_rogue (cast `/Game/RogueBoyard/Core/HUD_Rogue` (`PlayerController.GetHUD` (`GameplayStatics.GetPlayerController` 0))))
  (set `self.HUD` _ashud_rogue)
  (bind _asgm_rogue (cast `/Game/RogueBoyard/Core/GM_Rogue` (`GameplayStatics.GetGameMode`)))
  (set `self.GameMode` _asgm_rogue)
  (bind _returnvalue (`GameplayStatics.GetActorOfClass` "/Game/RogueBoyard/Props/BP_Door.BP_Door_C"))
  (set `self.Door` _returnvalue))

(event `self.ReceiveRoomEnter`
  (bind _door (`self.Door`))
  (bind (_gamemasterid _roomid _maxroomnb) (`/Game/RogueBoyard/Core/GM_Rogue.GetRoomInfo` (`self.GameMode`)))
  ;[1 1 1] Begin
  (`/Game/RogueBoyard/Core/HUD_Rogue.CE_ShowTitleCardSimon` (`self.HUD`) _gamemasterid _roomid _maxroomnb "Deactivate all levers and escape !")
  (`/Game/RogueBoyard/Props/BP_Door.CE_SetCam` (`self.Door`) (`self.RoomCamera`))
  (`KismetSystemLibrary.Delay` 3.0)
  (`/Game/RogueBoyard/Core/HUD_Rogue.CE_HideTitleCardSimon` (`self.HUD`))
  (add `/Game/RogueBoyard/Props/BP_Door.ED_Opened` _door (delegate `ED_Opened_Event`))
  (bind _asgm_rogue (cast `/Game/RogueBoyard/Core/GM_Rogue` (`GameplayStatics.GetGameMode`))
    (:`then`
      (`/Game/RogueBoyard/Core/GM_Rogue.PlacePlayers` _asgm_rogue))
    (:`CastFailed`
      _))
  (`/Game/RogueBoyard/Props/BP_Door.CE_OpenDoor` _door))

(event `ED_Opened_Event`
  ;[1 1 1] Begin
  (remove `/Game/RogueBoyard/Props/BP_Door.ED_Opened` (`self.Door`) (delegate `ED_Opened_Event`))
  (`/Game/RogueBoyard/Core/HUD_Rogue.CE_StartChrono` (`self.HUD`))
  (`KismetSystemLibrary.Delay` 3.0)
  (`self.BeginRoom`))

(event `self.ReceiveBeginRoom`
  ;[1 1 1] Begin
  (`/Game/RogueBoyard/Core/HUD_Rogue.CE_StartRoomTimer` (`self.HUD`) (`self.MaxRoomTime`))
  (bind _outactors (`GameplayStatics.GetAllActorsOfClass` "/Script/RogueBoyard.RogueTrap"))
  (for _array_element _outactors
    (`RogueTrap.Init` _array_element)))

(event `self.ReceiveEndRoom`
  (bind _door (`self.Door`))
  ;[1 1 1] End
  (`/Game/RogueBoyard/Core/HUD_Rogue.CE_EndRoomTimer` (`self.HUD`))
  (bind _outactors (`GameplayStatics.GetAllActorsOfClass` "/Script/RogueBoyard.RogueTrap"))
  (for _array_element _outactors
    (`RogueTrap.End` _array_element))
  (`/Game/RogueBoyard/Core/HUD_Rogue.CE_StartEndOfRoom` (`self.HUD`) (`self.bLizardsHasWon`))
  (`KismetSystemLibrary.Delay` 2.5)
  (add `/Game/RogueBoyard/Props/BP_Door.ED_Closed` _door (delegate `ED_Closed_Event`))
  (`/Game/RogueBoyard/Props/BP_Door.CE_CloseDoor` _door))

(event `ED_Closed_Event`
  ;[1 1 1] End
  (remove `/Game/RogueBoyard/Props/BP_Door.ED_Closed` (`self.Door`) (delegate `ED_Closed_Event`))
  (`self.RoomExit`))

(fn `UserConstructionScript`)