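; BP_Lever is a one-shot interactable lever that counts toward solving a riddle room.
; On BeginPlay it caches the GameMode's active room as a RogueRiddleRoom.
; The first Interact plays the lever animation and Wwise sound, then decrements the room's ThingsToValidate and prints a debug string.
; If the cached room is invalid at that moment, it re-fetches the active room before decrementing.
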(event `self.ReceiveBeginPlay`
  (bind _asgm_rogue (cast `/Game/RogueBoyard/Core/GM_Rogue` (`GameplayStatics.GetGameMode`)))
  (bind _asrogue_riddle_room (cast `RogueRiddleRoom` (`/Game/RogueBoyard/Core/GM_Rogue.ActiveRoom` _asgm_rogue)))
  (set `self.Room` _asrogue_riddle_room))

(event `/Game/RogueBoyard/BP/I_Interactable.Interact`
  (params (Character :type "/Game/RogueBoyard/Core/BP_Character Object Reference"))
  (`/Engine/EditorBlueprintResources/StandardMacros.DoOnce` false
    (:`Completed`
      (`SkeletalMeshComponent.PlayAnimation` (`self.Levier`) "/Game/RogueBoyard/GA/Assets/Meshs/msh_Levier/LevierAnim_Anim.LevierAnim_Anim" false)
      (`AkGameplayStatics.PostEvent` "/Game/WwiseAudio/Events/Default_Work_Unit/Items/Play_Lever.Play_Lever")
      (bind _room (`self.Room`)
        (:`then`
          (`/Engine/EditorBlueprintResources/StandardMacros.DecrementInt` (`RogueRiddleRoom.ThingsToValidate` _room)
            (:`  `
              _)))
        (:`else`
          (bind _asgm_rogue (cast `/Game/RogueBoyard/Core/GM_Rogue` (`GameplayStatics.GetGameMode`)))
          (bind _asrogue_riddle_room (cast `RogueRiddleRoom` (`/Game/RogueBoyard/Core/GM_Rogue.ActiveRoom` _asgm_rogue)))
          (bind _output_get (set `self.Room` _asrogue_riddle_room))
          (`/Engine/EditorBlueprintResources/StandardMacros.DecrementInt` (`RogueRiddleRoom.ThingsToValidate` _output_get)
            (:`  `
              _))))
      (`KismetSystemLibrary.PrintString` "Lever la vie dma mere"))))

(fn `UserConstructionScript`)