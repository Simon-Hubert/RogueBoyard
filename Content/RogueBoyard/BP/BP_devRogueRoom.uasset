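; BP_devRogueRoom is a development room Blueprint that drives the HUD when the room is entered.
; On BeginPlay it casts the first player controller's HUD to HUD_Rogue and caches it, printing a message if the cast fails.
; RoomEnter then tells that cached HUD to show the riddle room title card and start the chrono.
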(event `self.ReceiveBeginPlay`
  (bind _ashud_rogue (cast `/Game/RogueBoyard/Core/HUD_Rogue` (`PlayerController.GetHUD` (`GameplayStatics.GetPlayerController` 0)))
    (:`then`
      (set `self.As HUD Rogue` _ashud_rogue))
    (:`CastFailed`
      (`KismetSystemLibrary.PrintString` "cast failed"))))

(event `self.ReceiveRoomEnter`
  (bind _as_hud_rogue (`self.As HUD Rogue`))
  (`/Game/RogueBoyard/Core/HUD_Rogue.CE_ShowTitleCard` _as_hud_rogue (`/Game/RogueBoyard/Core/HUD_Rogue.RiddleRoomTC` _as_hud_rogue))
  (`/Game/RogueBoyard/Core/HUD_Rogue.CE_StartChrono` (`self.As HUD Rogue`)))

(fn `UserConstructionScript`)