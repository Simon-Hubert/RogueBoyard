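; BP_GrimoireLobby is a room Blueprint that runs the enter and exit sequence for the Grimoire lobby.
; On entry it points BP_Door at the room camera, places players through GM_Rogue and opens the door.
; Once the door opens, it initializes the Grimoire, hides the title card, starts the HUD room timer and begins the room.
; Ending stops room and vote timers, then waits on a one-shot door-closed binding before exiting.
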(event `self.ReceiveBeginPlay`
  (bind _ashud_rogue (cast `/Game/RogueBoyard/Core/HUD_Rogue` (`PlayerController.GetHUD` (`GameplayStatics.GetPlayerController` 0))))
  (set `self.HUD` _ashud_rogue)
  (bind _returnvalue (`GameplayStatics.GetActorOfClass` "/Game/RogueBoyard/Props/BP_Door.BP_Door_C"))
  (set `self.Door` _returnvalue))

(event `self.ReceiveRoomEnter`
  (bind _door (`self.Door`))
  (`/Game/RogueBoyard/Props/BP_Door.CE_SetCam` (`self.Door`) (`self.RoomCamera`))
  (add `/Game/RogueBoyard/Props/BP_Door.ED_Opened` _door (delegate `ED_Opened_Event`))
  (bind _asgm_rogue (cast `/Game/RogueBoyard/Core/GM_Rogue` (`GameplayStatics.GetGameMode`))
    (:`then`
      (`/Game/RogueBoyard/Core/GM_Rogue.PlacePlayers` _asgm_rogue))
    (:`CastFailed`
      _))
  (`/Game/RogueBoyard/Props/BP_Door.CE_OpenDoor` _door))

(event `ED_Opened_Event`
  (remove `/Game/RogueBoyard/Props/BP_Door.ED_Opened` (`self.Door`) (delegate `ED_Opened_Event`))
  (`RogueGrimoire.Init` (`self.Grimoire`))
  (`/Game/RogueBoyard/Core/HUD_Rogue.CE_HideTitleCardSimon` (`self.HUD`))
  (`/Game/RogueBoyard/Core/HUD_Rogue.CE_StartRoomTimer` (`self.HUD`) (`self.MaxRoomTime`))
  (`self.BeginRoom`))

(event `self.ReceiveEndRoom`
  (bind _door (`self.Door`))
  (`/Game/RogueBoyard/Core/HUD_Rogue.CE_EndRoomTimer` (`self.HUD`))
  (`/Game/RogueBoyard/Core/HUD_Rogue.CE_EndVoteTimer` (`self.HUD`))
  (add `/Game/RogueBoyard/Props/BP_Door.ED_Closed` _door (delegate `ED_Closed_Event`))
  (`/Game/RogueBoyard/Props/BP_Door.CE_CloseDoor` _door))

(event `ED_Closed_Event`
  (remove `/Game/RogueBoyard/Props/BP_Door.ED_Closed` (`self.Door`) (delegate `ED_Closed_Event`))
  (`self.RoomExit`))

(fn `UserConstructionScript`)