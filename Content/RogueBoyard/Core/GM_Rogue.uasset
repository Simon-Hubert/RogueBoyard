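; Game mode for RogueBoyard that runs the match loop, alternating lobby vote rooms and battle rooms before a final podium.
; The player voted in the lobby possesses the battle room's pawn against the other characters.
; Battle end rewards the winning side, resurrects players and shows progress before the next lobby or podium.
; RogueRoomSubsystem advances rooms, while each active room places players and supplies the camera that CameraWorldSubsystem uses to follow them.
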(event `Key|NumPadZero`
  (params (Key :type "Key Structure"))
  (:`Pressed`
    (`KismetSystemLibrary.PrintString` "Hello")
    (`RogueRoom.EndRoom` (`self.ActiveRoom`))))

(event `self.ReceiveBeginPlay`
  (bind _returnvalue (`GameplayStatics.GetPlayerController` 0))
  (`self.EnableInput` _returnvalue)
  (`AkGameplayStatics.PostEvent` "/Game/WwiseAudio/Events/Default_Work_Unit/PlayMusicInGame.PlayMusicInGame")
  (bind _ashud_rogue (cast `/Game/RogueBoyard/Core/HUD_Rogue` (`PlayerController.GetHUD` _returnvalue)))
  (`/Game/RogueBoyard/Core/HUD_Rogue.CE_ShowLoadingScreen` _ashud_rogue))

(event `self.StartBattleRoom`
  (`self.SetActiveRoom`)
  (`CameraWorldSubsystem.ClearFollowTarget` (subsystem `CameraWorldSubsystem`))
  (`self.UnPossessCharacter`)
  (`self.PlaceCamera`)
  (`RogueRoom.RoomEnter` (`self.ActiveRoom`))
  (`self.PlacePlayers`)
  (`self.SetCamera`))

(event `self.EndBattleRoom`
  (bind _returnvalue (subsystem `RogueRoomSubsystem`))
  (bind _roomwinners (`self.SelectWinningPlayers`))
  (`self.GiveRoomRewards` _roomwinners)
  (`self.UnPossessRoom`)
  (`self.Respawn All Player`)
  (`self.StopAllLoopingSounds`)
  (if (`self.bIsLastRoom`)
    (`self.CE_ShowLastRoomProgress`)
    (`KismetSystemLibrary.Delay` 4.0)
    (`self.PostLastRoom`)
    (`RogueRoomSubsystem.UnloadAllRooms` _returnvalue)
    (else
      (`RogueRoomSubsystem.NextRoom` _returnvalue)
      (`self.CE_ShowLastRoomProgress`)
      (`KismetSystemLibrary.Delay` 4.0)
      (`self.StartLobbyRoom`))))

(event `self.StartLobbyRoom`
  (`self.FirstCall`)
  (`CameraWorldSubsystem.ClearFollowTarget` (subsystem `CameraWorldSubsystem`))
  (set `self.ChosenPlayerIndex` -1)
  (`self.SetActiveRoom`)
  (`self.PlaceCamera`)
  (`RogueRoom.RoomEnter` (`self.ActiveRoom`))
  (`self.PlacePlayers`)
  (`self.SetCamera`))

(event `self.EndLobbyRoom`
  (`self.SetVotedPlayerIndex`)
  (`RogueRoomSubsystem.NextRoom` (subsystem `RogueRoomSubsystem`))
  (`self.StartBattleRoom`))

(event `self.ReceivePostLastRoom`
  (`CameraWorldSubsystem.ClearFollowTarget` (subsystem `CameraWorldSubsystem`))
  (set `self.ActiveRoom` (`self.PodiumManager`))
  (set `self.ChosenPlayerIndex` -1)
  (`self.PlaceCamera`)
  (`RogueRoom.RoomEnter` (`self.ActiveRoom`))
  (`self.PlacePlayers`)
  (`self.SetCamera`))

(event `self.ReceiveInitCharacters`
  (params (CharacterIndex :type Integer))
  (`self.InitCharacterMaterial` CharacterIndex))

(event `CE_ShowLastRoomProgress`
  (bind _returnvalue (subsystem `PlayerStatSubsystem`))
  (`PlayerController.SetViewTargetWithBlend` (`GameplayStatics.GetPlayerController` 0) (`self.CameraLastRoom`) 0.0 "VTBlend_Linear" 0.0 false)
  (`self.LastRoomCoinManager`
    (:`then`
      _)
    (:`else`
      (bind _returnvalue_2 (`GameplayStatics.GetActorOfClass` "/Game/RogueBoyard/Props/BP_PieceSpawnerManager.BP_PieceSpawnerManager_C"))
      (set `self.LastRoomCoinManager` _returnvalue_2)))
  (for (_array_element _array_index) (`PlayerStatSubsystem.GetPlayerBalance` _returnvalue)
    (`/Game/RogueBoyard/Props/BP_PieceSpawnerManager.CE_SpawnCoins` (`self.LastRoomCoinManager`) _array_index _array_element))
  (`PlayerStatSubsystem.ResetPlayerBalance` _returnvalue))

(fn `FirstCall`
  (if (not (`self.beginGame`))
    (set `self.beginGame` true)
    (`AkGameplayStatics.PostEvent` "/Game/WwiseAudio/Events/Default_Work_Unit/AMB/Play_AMB_Ambiance_LP.Play_AMB_Ambiance_LP")
    (bind _ashud_rogue (cast `/Game/RogueBoyard/Core/HUD_Rogue` (`PlayerController.GetHUD` (`GameplayStatics.GetPlayerController` 0))))
    (`/Game/RogueBoyard/Core/HUD_Rogue.CE_HideLoadingScreen` _ashud_rogue)))

(fn `GetRoomInfo`
  (returns (GameMasterID :type Integer) (RoomID :type Integer) (MaxRoomNB :type Integer))
  (return (`self.ChosenPlayerIndex`) (/ (+ (`RogueRoomSubsystem.ActiveRoomId` (subsystem `RogueRoomSubsystem`)) 1) 2) (defaults `RogueRoomSettings` "/Script/RogueBoyard.RogueRoomSettings")))

(fn `InitCharacterMaterial`
  (params (`Player Index` :type Integer))
  (locals (ListMaterial :type "Array of MaterialInstance Object Reference"))
  (bind (_dress _tongue _righteye _lefteye _ceinture _body _pants _collier `_auréole`) (break `/Game/RogueBoyard/Characters/ST_InstMaterial` (`|GetArrayItem` (`self.CharMaterials`) `Player Index`)))
  (bind _asbp_character (cast `/Game/RogueBoyard/Core/BP_Character` (`GameplayStatics.GetPlayerCharacter` `Player Index`)))
  (bind _mesh (`Character.Mesh` _asbp_character))
  (`PrimitiveComponent.SetMaterial` _mesh 0 _dress)
  (`PrimitiveComponent.SetMaterial` _mesh 1 _tongue)
  (`PrimitiveComponent.SetMaterial` _mesh 2 _righteye)
  (`PrimitiveComponent.SetMaterial` _mesh 3 _lefteye)
  (`PrimitiveComponent.SetMaterial` _mesh 4 _ceinture)
  (`PrimitiveComponent.SetMaterial` _mesh 5 _body)
  (`PrimitiveComponent.SetMaterial` _mesh 6 _pants)
  (`PrimitiveComponent.SetMaterial` _mesh 7 _collier)
  (`PrimitiveComponent.SetMaterial` _mesh 8 `_auréole`))

(fn `PlaceCamera`
  (`PlayerController.SetViewTargetWithBlend` (`GameplayStatics.GetPlayerController` 0) (`RogueRoom.RoomCamera` (`self.ActiveRoom`)) 0.0 "VTBlend_Linear" 0.0 false))

(fn `PlacePlayers`
  (for (_array_element _array_index) (`self.Characters`)
    (if (!= _array_index (`self.ChosenPlayerIndex`))
      (`RogueRoom.PlacePlayer` (`self.ActiveRoom`) _array_element _array_index))))

(fn `Respawn All Player`
  (for _array_element (`self.Characters`)
    (`RogueCharacter.Resurrect` _array_element))
  (`KismetSystemLibrary.PrintString` "Ressurected" false))

(fn `SelectWinningPlayers`
  (returns (RoomWinners :type "Array of RogueCharacter Object Reference"))
  (locals (Winners :type "Array of RogueCharacter Object Reference"))
  (bind _winners (`local.Winners`))
  (if (`RogueRoom.bLizardsHasWon` (`self.ActiveRoom`))
    (for _array_element (`self.Characters`)
      (if (and (!= (`RogueCharacter.PlayerIndex` _array_element) (`self.ChosenPlayerIndex`)) (`|EnumInequality` (`RogueCharacterStateMachine.CurrentStateID` (`RogueCharacter.StateMachine` _array_element)) "Dead"))
        (`KismetArrayLibrary.Array_Add` (`local.Winners`) _array_element)))
    (return (`local.Winners`))
    (else
      (`KismetArrayLibrary.Array_Add` _winners (`|GetArrayItem` (`self.Characters`) (`self.ChosenPlayerIndex`)))
      (return _winners))))

(fn `SetActiveRoom`
  (bind _output_get (set `self.ActiveRoom` (`|GetArrayItem` (`self.RoomManagers`) (`RogueRoomSubsystem.ActiveRoomId` (subsystem `RogueRoomSubsystem`)))))
  (`CameraWorldSubsystem.SetCamera` (subsystem `CameraWorldSubsystem`) (`RogueRoom.RoomCamera` _output_get) (`RogueRoom.RoomCameraZoomMax` _output_get) (`RogueRoom.RoomCameraZoomMin` _output_get)))

(fn `SetCamera`
  (if (< (`self.ChosenPlayerIndex`) 0)
    ;[0.427 0.7419 1] VoteRoom
    (for _array_element (`self.Characters`)
      (`CameraWorldSubsystem.AddFollowTarget` (subsystem `CameraWorldSubsystem`) _array_element))
    (else
      ;[1 0.5373 0.4915] BattleRoom
      (for (_array_element_2 _array_index) (`self.Characters`)
        (if (!= _array_index (`self.ChosenPlayerIndex`))
          (`CameraWorldSubsystem.AddFollowTarget` (subsystem `CameraWorldSubsystem`) _array_element_2))))))

(fn `SetVotedPlayerIndex`
  (bind _asrogue_lobby (cast `RogueLobby` (`self.ActiveRoom`)))
  (set `self.ChosenPlayerIndex` (`RogueLobby.ChosenPlayer` _asrogue_lobby)))

(fn `StopAllLoopingSounds`
  (`AkGameplayStatics.PostEvent` "/Game/WwiseAudio/Events/Default_Work_Unit/Traps/Flamethrower/Stop_Flamethrower_Loop.Stop_Flamethrower_Loop")
  (`AkGameplayStatics.PostEvent` "/Game/WwiseAudio/Events/Default_Work_Unit/Traps/GrindStone/Stop_SFX_Trap_Grindstone_LP.Stop_SFX_Trap_Grindstone_LP")
  (`AkGameplayStatics.PostEvent` "/Game/WwiseAudio/Events/Default_Work_Unit/Interactables/StopGrimoireLoop.StopGrimoireLoop")
  (`AkGameplayStatics.PostEvent` "/Game/WwiseAudio/Events/Default_Work_Unit/Traps/Lightning/StopLightningLoop.StopLightningLoop"))

(fn `UnPossessCharacter`
  (bind _roompawns (`self.RoomPawns`))
  (`RogueCharacter.UnPossessCharacter` (`|GetArrayItem` (`self.Characters`) (`self.ChosenPlayerIndex`)) (`|GetArrayItem` _roompawns (`KismetArrayLibrary.Array_LastIndex` _roompawns))))

(fn `UnPossessRoom`
  (bind _roompawns (`self.RoomPawns`))
  (`RogueRoomPawn.UnPossesRoom` (`|GetArrayItem` _roompawns (`KismetArrayLibrary.Array_LastIndex` _roompawns)) (`|GetArrayItem` (`self.Characters`) (`self.ChosenPlayerIndex`))))

(fn `UserConstructionScript`)