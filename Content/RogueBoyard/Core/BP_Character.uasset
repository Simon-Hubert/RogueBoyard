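; Player character Blueprint for the local multiplayer room-based game, handling movement, dash, charged push, item use, shop purchases, paralysis, death effects and resurrection.
; Input actions delegate to a state machine, while looping timers drive push charge, cooldowns and invincibility windows.
; A fully charged push fires automatically and briefly slows global time on a hit.
; Per-player DataTable colors tint Niagara effects, backed by Wwise audio, controller vibration and camera shakes.
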(event `self.ReceiveBeginPlay`
  (bind _ns_walk (`self.NS_Walk`))
  ;[1 1 1] Begin Play
  (bind _asgm_rogue (cast `/Game/RogueBoyard/Core/GM_Rogue` (`GameplayStatics.GetGameMode`)))
  (set `self.GameMode` _asgm_rogue)
  (add `RogueRoomSubsystem.OnNextRoomEvent` (subsystem `RogueRoomSubsystem`) (delegate `CE_OnNextRoom`))
  (set `self.speedNerfPrivate` 1.0)
  (`SceneComponent.SetVisibility` (`self.Widget`) false false)
  (bind _returnvalue (`|GetDataTableRow` "/Game/RogueBoyard/Characters/DT_Character.DT_Character" (select `int` (`self.PlayerIndex`) :`0` "J1" :`1` "J2" :`2` "J3" :`3` "J4" :!type "Name"))
    (:`then`
      (bind _returnvalue_2 (`KismetMathLibrary.Conv_ColorToLinearColor` (`.Player_Color_5_B78D15C3476A269E83BACD8E20EF06D1` (break `/Game/RogueBoyard/Characters/ST_Player` _returnvalue))))
      (`NiagaraComponent.SetVariableLinearColor` _ns_walk "Color01" _returnvalue_2)
      (bind (_returnvalue_r _returnvalue_g _returnvalue_b) (break `LinearColor` (/ _returnvalue_2 2.0)))
      (`NiagaraComponent.SetVariableLinearColor` _ns_walk "Color02" (make `LinearColor` _returnvalue_r _returnvalue_g _returnvalue_b))
      (`SceneComponent.SetVisibility` (`self.NS_Walk`) true false)
      (`SceneComponent.SetVisibility` (`self.W_AuctionFeedBack`) false false))))

(event `CE_OnNextRoom`
  ;[1 1 1] Begin Play
  (`self.SetCamera`))

(event `EnhancedInput|/Game/RogueBoyard/Inputs/InputDataPlaytest/IA_PTMoves`
  (params (ActionValue :type "Vector2D Structure") (ElapsedSeconds :type "Float (double-precision)") (TriggeredSeconds :type "Float (double-precision)") (InputAction :type "InputAction Object Reference" :default "/Game/RogueBoyard/Inputs/InputDataPlaytest/IA_PTMoves.IA_PTMoves"))
  (bind (_returnvalue_x _returnvalue_y _returnvalue_z) (`KismetMathLibrary.BreakVector` (`self.GetVelocity`)))
  (bind (_returnvalue_x_2 _returnvalue_y_2) (`KismetMathLibrary.BreakVector` (`self.GetVelocity`)))
  (bind _statemachine (`self.StateMachine`))
  (bind (_forwardvector_x _forwardvector_y _forwardvector_z) (`KismetMathLibrary.BreakVector` (`self.ForwardVector`)))
  (bind _speednerfprivate (`self.speedNerfPrivate`))
  (bind _buffinblackhole (`self.buffInBlackHole`))
  (bind _currentstate (`RogueCharacterStateMachine.CurrentState` _statemachine))
  ;[0.4104 1 0.4759] Movements
  (:`Triggered`
    (if (not (`self.Dashed`))
      (bind _newparam (`self.Threshold` ActionValue_X ActionValue_Y))
      (if _newparam
        (set `RogueCharacterStateMachine.Sticks` (0.0 0.0 0.0) _statemachine :!label _label)
        (else
          (set `RogueCharacterStateMachine.Sticks` (`KismetMathLibrary.MakeVector` ActionValue_X ActionValue_Y _returnvalue_z) _statemachine)
          (if (`self.bIsInBlackHole`)
            (`RogueCharacterState.Movement` _currentstate (* ActionValue_X _buffinblackhole) (* ActionValue_Y _buffinblackhole))
            (else
              (`RogueCharacterState.Movement` _currentstate (* ActionValue_X _speednerfprivate) (* ActionValue_Y _speednerfprivate))))
          (if (or (!= _returnvalue_x_2 0.0) (!= _returnvalue_y_2 0.0))
            (`SceneComponent.K2_SetWorldRotation` (`self.Mesh`) (`KismetMathLibrary.MakeRotFromX` (`KismetMathLibrary.MakeVector` _forwardvector_y (* _forwardvector_x -1.0) _forwardvector_z)) false false))))))
  (:`Completed`
    (goto _label)))

(event `self.ReceiveTick`
  (params (DeltaSeconds :type "Float (single-precision)"))
  (bind _charactermovement (`self.CharacterMovement`))
  (if (`SceneComponent.IsVisible` (`self.Widget`))
    (`self.Rotate_UI`))
  (if (`self.Dashed`)
    (if (>= (`KismetMathLibrary.VSize` (- (`self.K2_GetActorLocation`) (`self.StartDash`))) (`self.DashDistanceMax`))
      (set `MovementComponent.Velocity` (/ (`MovementComponent.Velocity` _charactermovement) 4) _charactermovement)
      (set `self.Dashed` false)
      (set `self.bDashed` false))))

(event `EnhancedInput|/Game/RogueBoyard/Inputs/InputDataPlaytest/IA_Dash`
  (params (ActionValue :type Boolean) (ElapsedSeconds :type "Float (double-precision)") (TriggeredSeconds :type "Float (double-precision)") (InputAction :type "InputAction Object Reference" :default "/Game/RogueBoyard/Inputs/InputDataPlaytest/IA_Dash.IA_Dash"))
  (bind _returnvalue (/ (`self.buffInBlackHole`) 2.0))
  (bind _currentstate (`RogueCharacterStateMachine.CurrentState` (`self.StateMachine`)))
  ;[0.1836 0.2918 1] Dash
  (:`Started`
    (if (and (not (`KismetSystemLibrary.K2_IsTimerActiveHandle` (`self.TimerDash`))) (not (`self.Dashed`)))
      (set `self.StartDash` (`self.K2_GetActorLocation`))
      (if (`self.bIsInBlackHole`)
        (bind _returnvalue_2 (`RogueCharacterState.Dash` _currentstate (/ (`KismetMathLibrary.BreakVector2D` (stale `EnhancedInput|/Game/RogueBoyard/Inputs/InputDataPlaytest/IA_PTMoves` ActionValue)) _returnvalue) (/ (`.Y` (`KismetMathLibrary.BreakVector2D` (stale `EnhancedInput|/Game/RogueBoyard/Inputs/InputDataPlaytest/IA_PTMoves` ActionValue))) _returnvalue)))
        (else
          (bind _returnvalue_3 (`RogueCharacterState.Dash` _currentstate (`.Y` (`KismetMathLibrary.BreakVector2D` (stale `EnhancedInput|/Game/RogueBoyard/Inputs/InputDataPlaytest/IA_PTMoves` ActionValue))) (`KismetMathLibrary.BreakVector2D` (stale `EnhancedInput|/Game/RogueBoyard/Inputs/InputDataPlaytest/IA_PTMoves` ActionValue))))))
      (set `self.Dashed` _returnvalue_2)
      (set `self.bDashed` _returnvalue_2)
      (if (and _returnvalue_3 (>= (`self.TimeDash`) 0.1))
        (`ActorComponent.K2_DestroyComponent` (`self.DashFX`))
        (else
          (`ControllerVibrationSubSystem.VibrationLightQuick` (subsystem `ControllerVibrationSubSystem`) (`GameplayStatics.GetPlayerController` (`self.PlayerIndex`)))
          (set `self.bIsInvincible` true)
          (bind _returnvalue_4 (`KismetSystemLibrary.K2_SetTimer` null "Invincibility" 0.1 true))
          (set `self.TimerDashInvincibility` _returnvalue_4)
          (bind _returnvalue_5 (`KismetSystemLibrary.K2_SetTimer` null "TimerDashSetting" 0.1 true))
          (set `self.TimerDash` _returnvalue_5)
          (`AkGameplayStatics.PostEvent` "/Game/WwiseAudio/Events/Default_Work_Unit/Player/Play_Dash.Play_Dash")
          (bind _returnvalue_6 (`NiagaraFunctionLibrary.SpawnSystemAttached` null (`self.Mesh`) "None" (0.0 0.0 0.0) (struct) "KeepRelativeOffset"))
          (bind _output_get (set `self.DashFX` _returnvalue_6))
          (bind _returnvalue_7 (`|GetDataTableRow` "/Game/RogueBoyard/Characters/DT_Character.DT_Character" (select `int` (`self.PlayerIndex`) :`0` "J1" :`1` "J2" :`2` "J3" :`3` "J4" :!type "Name"))
            (:`then`
              (`NiagaraComponent.SetVariableLinearColor` _output_get "LizzzardColor" (`KismetMathLibrary.Conv_ColorToLinearColor` (`.Player_Color_5_B78D15C3476A269E83BACD8E20EF06D1` (break `/Game/RogueBoyard/Characters/ST_Player` _returnvalue_7)))))))))))

(event `EnhancedInput|/Game/RogueBoyard/Inputs/InputDataPlaytest/IA_Interact`
  (params (ActionValue :type Boolean) (ElapsedSeconds :type "Float (double-precision)") (TriggeredSeconds :type "Float (double-precision)") (InputAction :type "InputAction Object Reference" :default "/Game/RogueBoyard/Inputs/InputDataPlaytest/IA_Interact.IA_Interact"))
  ;[1 1 1] Interact / Shop
  (:`Started`
    (bind _returnvalue (`RogueCharacterState.Interact` (`RogueCharacterStateMachine.CurrentState` (`self.StateMachine`))))
    (for _array_element _returnvalue
      (if (`KismetSystemLibrary.DoesImplementInterface` _array_element "/Game/RogueBoyard/BP/I_Interactable.I_Interactable_C")
        (message `/Game/RogueBoyard/BP/I_Interactable.Interact` _array_element self)))
    (`self.TryBuyItem`)))

(event `self.OnPushed`
  ;[1 1 1] Vibration OnPushed
  (`ControllerVibrationSubSystem.VibrationLightQuick` (subsystem `ControllerVibrationSubSystem`) (`GameplayStatics.GetPlayerController` (`self.PlayerIndex`))))

(event `self.CancelPushing_Implementation`
  (params (StateID :type "ERogueCharacterStateID Enum" :default "None"))
  (bind _fx (`self.FX`))
  (bind _timerpushing (`self.TimerPushing`))
  ;[0.979 0 1] Probablement le meilleur fix que j'ai fais sur un character de ma life
  (`KismetSystemLibrary.PrintString` "CANCELLLLLLLLLLLLL ANIMMMMMMMM")
  (set `self.CancelPush` true)
  (`/Engine/EditorBlueprintResources/StandardMacros.IsValid` _fx
    (:`Is Valid`
      (`ActorComponent.K2_DestroyComponent` _fx)
      (set `self.FX` null))
    (:`Is Not Valid`
      _))
  (`SkeletalMeshComponent.Stop` (`self.Mesh`))
  (if (`KismetSystemLibrary.K2_IsValidTimerHandle` _timerpushing)
    (`KismetSystemLibrary.K2_ClearAndInvalidateTimerHandle` _timerpushing))
  (set `self.ForcePush` 0.0)
  (set `self.speedNerfPrivate` 1.0)
  (set `self.TimerPushing` (struct))
  (set `self.TimeForce` 0.0)
  (`RogueCharacterStateMachine.ChangeState` (`self.StateMachine`) StateID)
  (set `self.CancelPush` false))

(event `EnhancedInput|/Game/RogueBoyard/Inputs/InputDataPlaytest/IA_Power`
  (params (ActionValue :type Boolean) (ElapsedSeconds :type "Float (double-precision)") (TriggeredSeconds :type "Float (double-precision)") (InputAction :type "InputAction Object Reference" :default "/Game/RogueBoyard/Inputs/InputDataPlaytest/IA_Power.IA_Power"))
  ;[0.3397 1 0.9302] Use Item
  (:`Started`
    (`RogueItemComponent.UseItem` (`self.UsableItem`))))

(event `FullCharged`
  ;[1 0.2747 0.2687] Push
  (`ControllerVibrationSubSystem.VibrationDegressive` (subsystem `ControllerVibrationSubSystem`) (`GameplayStatics.GetPlayerController` (`self.PlayerIndex`)))
  (bind _returnvalue (`RogueCharacterStatePushing.Pushing` (`self.RogueCharacterStatePushing`) (`PrimitiveComponent.GetOverlappingActors` (`self.Box`) null) (`self.ForcePush`)))
  (if _returnvalue
    (`GameplayStatics.PlayWorldCameraShake` "/Game/RogueBoyard/Core/Shaking/ShakeAfterPushingMAX.ShakeAfterPushingMAX_C" (`self.K2_GetActorLocation` (`RogueRoom.RoomCamera` (`RogueGameMode.ActiveRoom` (`self.GameMode`)))) 0.0 500.0)
    (`KismetSystemLibrary.Delay` 0.25)
    (`GameplayStatics.SetGlobalTimeDilation` 0.05)
    (`KismetSystemLibrary.Delay` (`self.FreezeScreenDuration`))
    (`GameplayStatics.SetGlobalTimeDilation` 1.0))
  (set `self.ForcePush` 0.0 :!label _label_2)
  (set `self.speedNerfPrivate` 1.0)
  (set `self.TimerPushing` (struct))
  (set `self.TimeForce` 0.0)
  (bind _returnvalue_2 (`KismetSystemLibrary.K2_SetTimer` null "TimerPushSetting" 0.1 true))
  (set `self.TimerPushCooldown` _returnvalue_2))

(event `EnhancedInput|/Game/RogueBoyard/Inputs/InputDataPlaytest/IA_Push`
  (params (ActionValue :type Boolean) (ElapsedSeconds :type "Float (double-precision)") (TriggeredSeconds :type "Float (double-precision)") (InputAction :type "InputAction Object Reference" :default "/Game/RogueBoyard/Inputs/InputDataPlaytest/IA_Push.IA_Push"))
  (bind _roguecharacterstatepushing (`self.RogueCharacterStatePushing`))
  (bind _statemachine (`self.StateMachine`))
  (bind _timerpushing (`self.TimerPushing`))
  (bind _currentstateid (`RogueCharacterStateMachine.CurrentStateID` _statemachine))
  ;[1 0.2747 0.2687] Push
  (:`Started`
    (if (and (not (`KismetSystemLibrary.K2_IsValidTimerHandle` (`self.TimerPushCooldown`))) (`|EnumInequality` _currentstateid "Dead") (`|EnumInequality` _currentstateid "Fall") (`|EnumInequality` _currentstateid "Stun"))
      (`RogueCharacterState.Push` (`RogueCharacterStateMachine.CurrentState` _statemachine))
      (if (`|EnumEquality` (`RogueCharacterStateMachine.CurrentStateID` _statemachine) "Pushing")
        (bind _returnvalue (`KismetSystemLibrary.K2_SetTimer` null "SetForcePush" 0.1 true))
        (set `self.TimerPushing` _returnvalue)
        (set `self.speedNerfPrivate` (`self.SpeedNerf`))
        (`self.SetColor_FX`))))
  (:`Completed`
    (`/Engine/EditorBlueprintResources/StandardMacros.IsValid` (`self.FX`)
      (:`Is Valid`
        (`ActorComponent.K2_DestroyComponent` (`self.FX`)))
      (:`Is Not Valid`
        _))
    (if (`KismetSystemLibrary.K2_IsValidTimerHandle` _timerpushing)
      (`KismetSystemLibrary.K2_ClearAndInvalidateTimerHandle` _timerpushing)
      (if (<= (`self.TimeForce`) (`RogueCharacterStatePushing.TimeMin` _roguecharacterstatepushing))
        (set `self.TimeForce` (`RogueCharacterStatePushing.MinForce` _roguecharacterstatepushing)))
      (if (not (`self.CancelPush`))
        (`ControllerVibrationSubSystem.VibrationLightQuick` (subsystem `ControllerVibrationSubSystem`) (`GameplayStatics.GetPlayerController` (`self.PlayerIndex`)))
        (`RogueCharacterStatePushing.Pushing` (`self.RogueCharacterStatePushing`) (`PrimitiveComponent.GetOverlappingActors` (`self.Box`) null) (`self.ForcePush`))
        (`GameplayStatics.PlayWorldCameraShake` "/Game/RogueBoyard/Core/Shaking/ShakeAfterPushing.ShakeAfterPushing_C" (`self.K2_GetActorLocation` (`RogueRoom.RoomCamera` (`RogueGameMode.ActiveRoom` (`self.GameMode`)))) 0.0 500.0)
        (goto _label_2)
        (else
          (goto _label_2))))))

(event `EnhancedInput|/Game/RogueBoyard/Inputs/InputDataPlaytest/IA_Resurect_1`
  (params (ActionValue :type Boolean) (ElapsedSeconds :type "Float (double-precision)") (TriggeredSeconds :type "Float (double-precision)") (InputAction :type "InputAction Object Reference" :default "/Game/RogueBoyard/Inputs/InputDataPlaytest/IA_Resurect_1.IA_Resurect_1"))
  ;[1 0.8821 0.3875] Ressurect
  (:`Triggered`
    (if (and ActionValue (stale `EnhancedInput|/Game/RogueBoyard/Inputs/InputDataPlaytest/IA_Resurect_2` ActionValue)) :!label _label_3
      (`RogueCharacterState.Resurrect` (`RogueCharacterStateMachine.CurrentState` (`self.StateMachine`)))
      (bind _asrogue_character_state_dead (cast `RogueCharacterStateDead` (`RogueCharacterStateMachine.CurrentState` (`self.StateMachine`))))
      (`SkeletalMeshComponent.PlayAnimation` (`self.Mesh`) (`RogueCharacterStateDead.ResurectMontage` _asrogue_character_state_dead) false))))

(event `EnhancedInput|/Game/RogueBoyard/Inputs/InputDataPlaytest/IA_Resurect_2`
  (params (ActionValue :type Boolean) (ElapsedSeconds :type "Float (double-precision)") (TriggeredSeconds :type "Float (double-precision)") (InputAction :type "InputAction Object Reference" :default "/Game/RogueBoyard/Inputs/InputDataPlaytest/IA_Resurect_2.IA_Resurect_2"))
  ;[1 0.8821 0.3875] Ressurect
  (:`Triggered`
    (goto _label_3)))

(event `self.TriggerFinishPushed`
  (bind _returnvalue (`NiagaraFunctionLibrary.SpawnSystemAtLocation` "/Game/RogueBoyard/VFX/NS_Poof.NS_Poof" (`SceneComponent.K2_GetComponentLocation` (`self.Mesh`))))
  (bind _returnvalue_2 (`|GetDataTableRow` "/Game/RogueBoyard/Characters/DT_Character.DT_Character" (select `int` (`self.PlayerIndex`) :`0` "J1" :`1` "J2" :`2` "J3" :`3` "J4" :!type "Name"))
    (:`then`
      (`NiagaraComponent.SetVariableLinearColor` _returnvalue "Color01" (`KismetMathLibrary.Conv_ColorToLinearColor` (`.Player_Color_5_B78D15C3476A269E83BACD8E20EF06D1` (break `/Game/RogueBoyard/Characters/ST_Player` _returnvalue_2))))
      (`NiagaraComponent.SetVariableLinearColor` _returnvalue "Color02" (make `LinearColor` 0.1 0.1 0.1 1.0)))))

(event `CE_DeathAnim`
  ;[1 1 1] Le décès à la vanille
  (`AkGameplayStatics.PostEvent` "/Game/WwiseAudio/Events/Default_Work_Unit/Player/Play_Despawn.Play_Despawn"))

(event `CE_EnDeathAnim`
  (bind _mesh (`self.Mesh`))
  (bind (_returnvalue_roll _returnvalue_pitch _returnvalue_yaw) (`KismetMathLibrary.BreakRotator` (`SceneComponent.GetSocketRotation` _mesh "CentreAureole")))
  ;[1 1 1] Le décès à la vanille
  (`NiagaraFunctionLibrary.SpawnSystemAtLocation` "/Game/RogueBoyard/VFX/Systems/Player/NS_Push.NS_Push" (`SceneComponent.GetSocketLocation` _mesh "CentreAureole") (`KismetMathLibrary.MakeRotator` -90.0 0.0 _returnvalue_yaw))
  (`ControllerVibrationSubSystem.VibrationLightQuick` (subsystem `ControllerVibrationSubSystem`) (`GameplayStatics.GetPlayerController` (`self.PlayerIndex`)))
  (`self.K2_SetActorLocation` (99999.0 99999.0 99999.0))
  (`GameplayStatics.PlayWorldCameraShake` "/Game/RogueBoyard/Core/Shaking/ShakeAfterPushing.ShakeAfterPushing_C" (`self.K2_GetActorLocation` (`RogueRoom.RoomCamera` (`RogueGameMode.ActiveRoom` (`self.GameMode`)))) 0.0 500.0))

(event `self.ReceiveInvincibilityAfterParalysis`
  ;[0.3805 1 0.3904] Paralysis
  (bind _returnvalue (`KismetSystemLibrary.K2_SetTimer` null "Invincibility_AfterParalysis" 0.1 true))
  (set `self.Timer_InvincibilityAfterParalisys` _returnvalue))

(event `self.Box.OnComponentBeginOverlap`
  (params (OverlappedComponent :type "PrimitiveComponent Object Reference") (OtherActor :type "Actor Object Reference") (OtherComp :type "PrimitiveComponent Object Reference") (OtherBodyIndex :type Integer) (bFromSweep :type Boolean) (SweepResult :type "HitResult Structure (by ref)"))
  ;[1 0.3091 0.01177] UI
  (if (`KismetSystemLibrary.DoesImplementInterface` OtherActor "/Game/RogueBoyard/BP/I_Interactable.I_Interactable_C")
    (`SceneComponent.SetVisibility` (`self.Widget`) true false)))

(event `self.Box.OnComponentEndOverlap`
  (params (OverlappedComponent :type "PrimitiveComponent Object Reference") (OtherActor :type "Actor Object Reference") (OtherComp :type "PrimitiveComponent Object Reference") (OtherBodyIndex :type Integer))
  ;[1 0.3091 0.01177] UI
  (if (`KismetSystemLibrary.DoesImplementInterface` OtherActor "/Game/RogueBoyard/BP/I_Interactable.I_Interactable_C")
    (`SceneComponent.SetVisibility` (`self.Widget`) false false)))

(event `self.RogueCharacterStateRun.OnStartMoving`
  ;[1 0.4919 0.5337] Event Start/Stop moving
  (`NiagaraComponent.SetVariableFloat` (`self.NS_Walk`) "SpawnRate" 1.0))

(event `self.RogueCharacterStateRun.OnStopMoving`
  ;[1 0.4919 0.5337] Event Start/Stop moving
  (`NiagaraComponent.SetVariableFloat` (`self.NS_Walk`) "SpawnRate" 0.0))

(event `self.RogueCharacterStatePushing.OnStartMoving`
  ;[1 0.4919 0.5337] Event Start/Stop moving
  (`NiagaraComponent.SetVariableFloat` (`self.NS_Walk`) "SpawnRate" 1.0))

(event `self.RogueCharacterStatePushing.OnStopMoving`
  ;[1 0.4919 0.5337] Event Start/Stop moving
  (`NiagaraComponent.SetVariableFloat` (`self.NS_Walk`) "SpawnRate" 0.0))

(fn `Invincibility`
  (bind _output_get (set `self.DashTimeInvincibility` (+ (`self.DashTimeInvincibility`) 0.1)))
  (if (>= _output_get (`self.TimeInvincibleDash`))
    (set `self.bIsInvincible` false)
    (`KismetSystemLibrary.K2_ClearAndInvalidateTimerHandle` (`self.TimerDashInvincibility`))
    (set `self.TimerDashInvincibility` (struct))))

(fn `Invincibility_AfterParalysis`
  (set `self.ParalysisInvincibility_TIme` (+ (`self.ParalysisInvincibility_TIme`) 0.1))
  (if (>= (`self.ParalysisInvincibility_TIme`) (`self.CantStunTime`))
    (set `self.Paralized` false)
    (set `RogueCharacterStateStun.bParalized` false (`self.RogueCharacterStateStun`))
    (`KismetSystemLibrary.K2_ClearAndInvalidateTimerHandle` (`self.Timer_InvincibilityAfterParalisys`))
    (set `self.Timer_InvincibilityAfterParalisys` (struct))
    (set `self.ParalysisInvincibility_TIme` 0.0)))

(fn `Paralysis`
  (params (ParalysisTime :type "Float (double-precision)"))
  (bind _statemachine (`self.StateMachine`))
  (`ControllerVibrationSubSystem.VibrationLightContinuous` (subsystem `ControllerVibrationSubSystem`) (`GameplayStatics.GetPlayerController` (`self.PlayerIndex`)))
  (if (`|EnumEquality` (`RogueCharacterStateMachine.CurrentStateID` _statemachine) "Dead")
    _
    (elif (not (`self.Paralized`))
      (if (`|EnumEquality` (`RogueCharacterStateMachine.CurrentStateID` _statemachine) "Pushing")
        (`parent.CancelPushing_Implementation` "Stun")
        (set `self.Paralized` true)
        (`RogueCharacterStateStun.Paralysis` (`self.RogueCharacterStateStun`) ParalysisTime)
        (else
          (set `self.Paralized` true)
          (`RogueCharacterStateMachine.ChangeState` _statemachine "Stun")
          (`RogueCharacterStateStun.Paralysis` (`self.RogueCharacterStateStun`) ParalysisTime)))
      (`GameplayStatics.PlayWorldCameraShake` "/Game/RogueBoyard/Core/Shaking/ShakeAfterParalysis.ShakeAfterParalysis_C" (`self.K2_GetActorLocation` (`RogueRoom.RoomCamera` (`RogueGameMode.ActiveRoom` (`self.GameMode`)))) 0.0 500.0))))

(fn `Rotate_UI`
  (bind _w_auctionfeedback (`self.W_AuctionFeedBack`))
  (bind _widget (`self.Widget`))
  (bind _returnvalue (`self.K2_GetActorLocation` (`CameraWorldSubsystem.CurrentCamera` (subsystem `CameraWorldSubsystem`))))
  (`SceneComponent.K2_SetWorldRotation` _widget (`KismetMathLibrary.FindLookAtRotation` (`SceneComponent.K2_GetComponentLocation` _widget) _returnvalue) false false)
  (`SceneComponent.K2_SetWorldRotation` _w_auctionfeedback (`KismetMathLibrary.FindLookAtRotation` (`SceneComponent.K2_GetComponentLocation` _w_auctionfeedback) _returnvalue) false false))

(fn `SetColor_FX`
  (bind _returnvalue (`NiagaraFunctionLibrary.SpawnSystemAttached` "/Game/RogueBoyard/VFX/Systems/Player/NS_PlayerCharge.NS_PlayerCharge" (`self.Mesh`) "CentreAureole" (0.0 0.0 0.0) (struct) "KeepRelativeOffset"))
  (bind _returnvalue_2 (`|GetDataTableRow` "/Game/RogueBoyard/Characters/DT_Character.DT_Character" (select `int` (`self.PlayerIndex`) :`0` "J1" :`1` "J2" :`2` "J3" :`3` "J4" :!type "Name"))
    (:`then`
      (`NiagaraComponent.SetVariableLinearColor` _returnvalue "Color" (`KismetMathLibrary.Conv_ColorToLinearColor` (`.Player_Color_5_B78D15C3476A269E83BACD8E20EF06D1` (break `/Game/RogueBoyard/Characters/ST_Player` _returnvalue_2))))
      (set `self.FX` _returnvalue))))

(fn `SetForcePush`
  (bind _roguecharacterstatepushing (`self.RogueCharacterStatePushing`))
  (bind _roguecharacterstatepushing_2 (`self.RogueCharacterStatePushing`))
  (set `self.TimeForce` (+ (`self.TimeForce`) 0.1))
  (if (>= (`self.TimeForce`) (`RogueCharacterStatePushing.TimeMax` _roguecharacterstatepushing_2))
    (set `self.ForcePush` (`RogueCharacterStatePushing.MaxForce` _roguecharacterstatepushing_2))
    (`KismetSystemLibrary.K2_ClearAndInvalidateTimerHandle` (`self.TimerPushing`))
    (set `self.TimerPushing` (struct))
    (`self.FullCharged`)
    (else
      (set `self.ForcePush` (`KismetMathLibrary.Lerp` (`RogueCharacterStatePushing.MinForce` _roguecharacterstatepushing) (`RogueCharacterStatePushing.MaxForce` _roguecharacterstatepushing) (`self.InverseLerp` (`RogueCharacterStatePushing.TimeMin` _roguecharacterstatepushing) (`RogueCharacterStatePushing.TimeMax` _roguecharacterstatepushing) (`self.TimeForce`)))))))

(fn `Threshold`
  (params (X :type "Float (double-precision)") (Y :type "Float (double-precision)"))
  (returns (NewParam :type Boolean))
  (bind _stickthreshold (`self.StickThreshold`))
  (return (and (and (<= X _stickthreshold) (>= X (* _stickthreshold -1.0))) (and (<= Y _stickthreshold) (>= Y (* -1.0 _stickthreshold))))))

(fn `TimerDashSetting`
  (bind _output_get (set `self.TimeDash` (+ (`self.TimeDash`) 0.1)))
  (if (> _output_get (`RogueCharacterStateDash.DashCoolDown` (`self.RogueCharacterStateDash`)))
    (`KismetSystemLibrary.K2_ClearAndInvalidateTimerHandle` (`self.TimerDash`))
    (set `self.TimerDash` (struct))
    (set `self.TimeDash` 0.0)))

(fn `TimerPushSetting`
  (bind _output_get (set `self.TimePush` (+ (`self.TimePush`) 0.1)))
  (if (> _output_get (`RogueCharacterStatePushing.PushingCoolDown` (`self.RogueCharacterStatePushing`)))
    (`KismetSystemLibrary.K2_ClearAndInvalidateTimerHandle` (`self.TimerPushCooldown`))
    (set `self.TimerPushCooldown` (struct))
    (set `self.TimePush` 0.0)))

(fn `TryBuyItem`
  (returns (Success :type Boolean))
  (bind _overlappingactors (`PrimitiveComponent.GetOverlappingActors` (`self.Box`) "/Game/RogueBoyard/Props/BP_Shop.BP_Shop_C"))
  (if (`KismetArrayLibrary.Array_IsNotEmpty` _overlappingactors)
    (bind _asbp_shop (cast `/Game/RogueBoyard/Props/BP_Shop` (`|GetArrayItem` _overlappingactors))
      (:`then`
        (bind _returnvalue (`RogueShop.BuyItem` _asbp_shop))
        (`RoguePurse.Spend` (`self.Purse`) (`.Price` (break `ShopItemData` _returnvalue)))
        (bind _returnvalue_2 (`|GenericCreateObject` (`.ItemObject` (break `ShopItemData` _returnvalue))))
        (`/Engine/EditorBlueprintResources/StandardMacros.IsValid` _returnvalue_2
          (:`Is Valid`
            (`RogueItemComponent.SetCurrentItem` (`self.UsableItem`) _returnvalue_2)
            (return true))
          (:`Is Not Valid`
            (`KismetSystemLibrary.PrintString` "Bought Item Not Valid" false)
            (return false))))
      (:`CastFailed`
        (`KismetSystemLibrary.PrintString` "NoShop" false)
        (return false)))
    (else
      (`KismetSystemLibrary.PrintString` "No Buyable Item in range" false)
      (return false))))

(fn `UserConstructionScript`)