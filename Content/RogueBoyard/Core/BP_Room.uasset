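; BP_Room is a room that routes a player's gamepad input to the elements bound to each control.
; Enhanced Input events loop over one array per stick, face button or trigger, forwarding stick axes through Trigger and presses through Started/Stopped.
; Presses also send a quick light vibration to that player's controller: face buttons once per bound element on Started, triggers on every Triggered event, even with nothing bound.
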(event `EnhancedInput|/Game/RogueBoyard/Inputs/InputData/IA_GamePadMoves`
  (params (ActionValue :type "Vector2D Structure") (ElapsedSeconds :type "Float (double-precision)") (TriggeredSeconds :type "Float (double-precision)") (InputAction :type "InputAction Object Reference" :default "/Game/RogueBoyard/Inputs/InputData/IA_GamePadMoves.IA_GamePadMoves"))
  ;[1 1 1] Right Stick
  (:`Triggered`
    (for _array_element (`self.RightStick`) :!label _label
      (`TrapsInput.Trigger` _array_element (`KismetMathLibrary.MakeVector` ActionValue_X ActionValue_Y))))
  (:`Completed`
    (goto _label)))

(event `EnhancedInput|/Game/RogueBoyard/Inputs/InputDataPlaytest/IA_PTMoves`
  (params (ActionValue :type "Vector2D Structure") (ElapsedSeconds :type "Float (double-precision)") (TriggeredSeconds :type "Float (double-precision)") (InputAction :type "InputAction Object Reference" :default "/Game/RogueBoyard/Inputs/InputDataPlaytest/IA_PTMoves.IA_PTMoves"))
  ;[1 1 1] Left Stick
  (:`Triggered`
    (for _array_element (`self.LeftStick`) :!label _label_2
      (`TrapsInput.Trigger` _array_element (`KismetMathLibrary.MakeVector` ActionValue_X ActionValue_Y))))
  (:`Completed`
    (goto _label_2)))

(event `EnhancedInput|/Game/RogueBoyard/Inputs/InputDataPlaytest/IA_Dash`
  (params (ActionValue :type Boolean) (ElapsedSeconds :type "Float (double-precision)") (TriggeredSeconds :type "Float (double-precision)") (InputAction :type "InputAction Object Reference" :default "/Game/RogueBoyard/Inputs/InputDataPlaytest/IA_Dash.IA_Dash"))
  (bind _rightbutton (`self.RightButton`))
  ;[1 1 1] Right Button
  (:`Started`
    (for _array_element _rightbutton
      (`TrapsInput.Started` _array_element)
      (`ControllerVibrationSubSystem.VibrationLightQuick` (subsystem `ControllerVibrationSubSystem`) (`GameplayStatics.GetPlayerController` (`RogueCharacter.PlayerIndex` (`self.Player`))))))
  (:`Canceled`
    (for _array_element_2 _rightbutton :!label _label_3
      (`TrapsInput.Stopped` _array_element_2)))
  (:`Completed`
    (goto _label_3)))

(event `EnhancedInput|/Game/RogueBoyard/Inputs/InputDataPlaytest/IA_Interact`
  (params (ActionValue :type Boolean) (ElapsedSeconds :type "Float (double-precision)") (TriggeredSeconds :type "Float (double-precision)") (InputAction :type "InputAction Object Reference" :default "/Game/RogueBoyard/Inputs/InputDataPlaytest/IA_Interact.IA_Interact"))
  (bind _bottombutton (`self.BottomButton`))
  ;[1 1 1] Bottom Button
  (:`Started`
    (for _array_element _bottombutton
      (`TrapsInput.Started` _array_element)
      (`ControllerVibrationSubSystem.VibrationLightQuick` (subsystem `ControllerVibrationSubSystem`) (`GameplayStatics.GetPlayerController` (`RogueCharacter.PlayerIndex` (`self.Player`))))))
  (:`Canceled`
    (for _array_element_2 _bottombutton :!label _label_4
      (`TrapsInput.Stopped` _array_element_2)))
  (:`Completed`
    (goto _label_4)))

(event `EnhancedInput|/Game/RogueBoyard/Inputs/InputDataPlaytest/IA_Push`
  (params (ActionValue :type Boolean) (ElapsedSeconds :type "Float (double-precision)") (TriggeredSeconds :type "Float (double-precision)") (InputAction :type "InputAction Object Reference" :default "/Game/RogueBoyard/Inputs/InputDataPlaytest/IA_Push.IA_Push"))
  (bind _leftbutton (`self.LeftButton`))
  ;[1 1 1] Left Button
  (:`Started`
    (for _array_element _leftbutton
      (`TrapsInput.Started` _array_element)
      (`ControllerVibrationSubSystem.VibrationLightQuick` (subsystem `ControllerVibrationSubSystem`) (`GameplayStatics.GetPlayerController` (`RogueCharacter.PlayerIndex` (`self.Player`))))))
  (:`Canceled`
    (for _array_element_2 _leftbutton :!label _label_5
      (`TrapsInput.Stopped` _array_element_2)))
  (:`Completed`
    (goto _label_5)))

(event `EnhancedInput|/Game/RogueBoyard/Inputs/InputDataPlaytest/IA_Resurect_1`
  (params (ActionValue :type Boolean) (ElapsedSeconds :type "Float (double-precision)") (TriggeredSeconds :type "Float (double-precision)") (InputAction :type "InputAction Object Reference" :default "/Game/RogueBoyard/Inputs/InputDataPlaytest/IA_Resurect_1.IA_Resurect_1"))
  (bind _lefttrigger (`self.LeftTrigger`))
  ;[1 1 1] Left Trigger
  (:`Triggered`
    (`ControllerVibrationSubSystem.VibrationLightQuick` (subsystem `ControllerVibrationSubSystem`) (`GameplayStatics.GetPlayerController` (`RogueCharacter.PlayerIndex` (`self.Player`)))))
  (:`Started`
    (for _array_element _lefttrigger
      (`TrapsInput.Started` _array_element)))
  (:`Canceled`
    (for _array_element_2 _lefttrigger :!label _label_6
      (`TrapsInput.Stopped` _array_element_2)))
  (:`Completed`
    (goto _label_6)))

(event `EnhancedInput|/Game/RogueBoyard/Inputs/InputDataPlaytest/IA_Resurect_2`
  (params (ActionValue :type Boolean) (ElapsedSeconds :type "Float (double-precision)") (TriggeredSeconds :type "Float (double-precision)") (InputAction :type "InputAction Object Reference" :default "/Game/RogueBoyard/Inputs/InputDataPlaytest/IA_Resurect_2.IA_Resurect_2"))
  (bind _righttrigger (`self.RightTrigger`))
  ;[1 1 1] Right Trigger
  (:`Triggered`
    (`ControllerVibrationSubSystem.VibrationLightQuick` (subsystem `ControllerVibrationSubSystem`) (`GameplayStatics.GetPlayerController` (`RogueCharacter.PlayerIndex` (`self.Player`)))))
  (:`Started`
    (for _array_element _righttrigger
      (`TrapsInput.Started` _array_element)))
  (:`Canceled`
    (for _array_element_2 _righttrigger :!label _label_7
      (`TrapsInput.Stopped` _array_element_2)))
  (:`Completed`
    (goto _label_7)))

(event `EnhancedInput|/Game/RogueBoyard/Inputs/InputDataPlaytest/IA_Power`
  (params (ActionValue :type Boolean) (ElapsedSeconds :type "Float (double-precision)") (TriggeredSeconds :type "Float (double-precision)") (InputAction :type "InputAction Object Reference" :default "/Game/RogueBoyard/Inputs/InputDataPlaytest/IA_Power.IA_Power"))
  (bind _topbutton (`self.TopButton`))
  ;[1 1 1] Top Button
  (:`Started`
    (for _array_element _topbutton
      (`TrapsInput.Started` _array_element)
      (`ControllerVibrationSubSystem.VibrationLightQuick` (subsystem `ControllerVibrationSubSystem`) (`GameplayStatics.GetPlayerController` (`RogueCharacter.PlayerIndex` (`self.Player`))))))
  (:`Canceled`
    (for _array_element_2 _topbutton :!label _label_8
      (`TrapsInput.Stopped` _array_element_2)))
  (:`Completed`
    (goto _label_8)))

(fn `UserConstructionScript`)